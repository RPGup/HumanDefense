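; BP_Human is a defender unit that detects enemies around itself, fights them and walks back to its spawn point.
; A delayed Search loop sphere-traces attack range, then move range if movement is allowed, to attack, chase or return.
; FindFirstEnemy targets by distance to BP_Base, using a stored Destance threshold it never resets.
; Attacks repeat a montage whose notify calls AttackTo, which is empty here.
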(event `self.ReceiveBeginPlay`
  (bind _outactors (`GameplayStatics.GetAllActorsOfClass` "/Game/HumanDenfense/Aline/Base/BP_Base.BP_Base_C"))
  (set `self.Ref_Base` (`|GetArrayItem` _outactors))
  (`self.Search`)
  (set `self.wordlocation` (`self.K2_GetActorLocation`)))

(event `Search`
  (bind _returnvalue (`self.K2_GetActorLocation`))
  (bind _returnvalue_2 (`self.K2_GetActorLocation`))
  (bind _ref_searchedenemy (`self.Ref_SearchedEnemy`))
  (`KismetSystemLibrary.Delay` (`self.AtackDelay`))
  (if (not (`self.isbacking?`))
    (bind (_outhits _returnvalue_3) (`KismetSystemLibrary.SphereTraceMultiForObjects` :`Start` _returnvalue_2 :`End` _returnvalue_2 :`Radius` (`self.AttackRange`) :`ObjectTypes` (`|MakeArray` "ObjectTypeQuery8" :!type "EObjectTypeQuery Enum") :`DrawDebugType` "ForDuration"))
    (if _returnvalue_3
      (`KismetArrayLibrary.Array_Clear` (`self.Ref_SearchedEnemy`))
      (for _array_element _outhits
        (`KismetArrayLibrary.Array_Add` (`self.Ref_SearchedEnemy`) (`.HitActor` (`GameplayStatics.BreakHitResult` _array_element))))
      (if (> (`KismetArrayLibrary.Array_Length` (`self.Ref_SearchedEnemy`)) 0)
        (bind _issearched (`self.FindFirstEnemy`))
        (if _issearched
          (`self.AttackNormal`)
          (else
            (`self.Search` :!label _label)))
        (else
          (goto _label)))
      (elif (and (`self.CanMove`) (`self.IsNotMoving`))
        (bind (_outhits_2 _returnvalue_4) (`KismetSystemLibrary.SphereTraceMultiForObjects` :`Start` _returnvalue :`End` _returnvalue :`Radius` (`self.MoveRange`) :`ObjectTypes` (`|MakeArray` "ObjectTypeQuery8" :!type "EObjectTypeQuery Enum") :`DrawDebugType` "ForDuration"))
        (if _returnvalue_4
          (`KismetArrayLibrary.Array_Clear` (`self.Ref_SearchedEnemyMove`))
          (for _array_element_2 _outhits_2
            (`KismetArrayLibrary.Array_Add` _ref_searchedenemy (`.HitActor` (`GameplayStatics.BreakHitResult` _array_element_2)))
            (`KismetSystemLibrary.PrintString` (`KismetStringLibrary.Conv_IntToString` (`KismetArrayLibrary.Array_Length` _ref_searchedenemy))))
          (if (> (`KismetArrayLibrary.Array_Length` (`self.Ref_SearchedEnemy`)) 0)
            (bind _issearched_2 (`self.FindFirstEnemy`))
            (if _issearched_2
              (`self.MoveTo`)
              (`KismetSystemLibrary.PrintString` "Move")
              (else
                (`self.Search` :!label _label_2)))
            (else
              (goto _label_2)))
          (else
            (`self.Back`)))
        (else
          (`self.Search`))))))

(event `AttackNormal`
  (bind _ref_firstenemy (`self.Ref_FirstEnemy`))
  (bind (_returnvalue_roll _returnvalue_pitch _returnvalue_yaw) (`KismetMathLibrary.BreakRotator` (`KismetMathLibrary.FindLookAtRotation` (`self.K2_GetActorLocation`) (`self.K2_GetActorLocation` (`self.Ref_FirstEnemy`)))))
  (`self.K2_SetActorRotation` (`KismetMathLibrary.MakeRotator` 0.0 0.0 _returnvalue_yaw))
  (`|PlayMontage` (`self.Mesh`) (`self.Ref_Montage`) 1.0 0.0 (`self.StartSection`)
    (:`then`
      (set `self.isAttacking` true))
    (:`OnCompleted`
      (`KismetSystemLibrary.Delay` (`self.AtackDelay`))
      (if (`KismetSystemLibrary.IsValid` _ref_firstenemy)
        (if (> (`KismetMathLibrary.VSize` (- (`self.K2_GetActorLocation` _ref_firstenemy) (`self.K2_GetActorLocation` self))) (`self.AttackRange`))
          (`self.Search` :!label _label_3)
          (set `self.isAttacking` false)
          (else
            (`self.AttackNormal`)))
        (else
          (goto _label_3))))
    (:`OnNotifyBegin`
      (`self.AttackTo`))))

(event `AttackTo`)

(event `MoveTo`
  (set `self.IsNotMoving` false)
  (`|AIMoveTo` self (0.0 0.0 0.0) (`self.Ref_FirstEnemy`) (`self.AttackRange`)
    (:`then`
      (`self.Search`))
    (:`OnSuccess`
      (set `self.IsNotMoving` true :!label _label_4))
    (:`OnFail`
      (goto _label_4))))

(event `Back`
  (`|AIMoveTo` self (`self.wordlocation`) null 0.0
    (:`then`
      (set `self.isbacking?` true))
    (:`OnSuccess`
      (set `self.isbacking?` false :!label _label_5)
      (`self.Search`))
    (:`OnFail`
      (goto _label_5))))

(fn `FindFirstEnemy`
  (returns (IsSearched :type Boolean))
  (locals (Destance :type "Float (double-precision)" :default 9999.0))
  (for _array_element (`self.Ref_SearchedEnemy`)
    (bind _returnvalue (`KismetMathLibrary.VSize` (- (`self.K2_GetActorLocation` _array_element) (`self.K2_GetActorLocation` (`self.Ref_Base`)))))
    (if (<= _returnvalue (`local.Destance`))
      (set `local.Destance` _returnvalue)
      (set `self.Ref_FirstEnemy` _array_element)))
  (return (`KismetSystemLibrary.IsValid` (`self.Ref_FirstEnemy`))))

(fn `UserConstructionScript`)