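; BP_NomalBullet is a homing projectile that chases the actor held in RefAttacking.
; Each Tick it takes a swept step of Speed along the normalized direction to that actor, without scaling by delta time, and destroys itself once the reference is invalid.
; Box overlaps forward the other actor to an Overlap event, which is empty here, so this Blueprint applies no hit effect itself.
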(event `self.ReceiveBeginPlay`)

(event `self.ReceiveTick`
  (params (DeltaSeconds :type "Float (single-precision)"))
  (bind _ref_attacking (`self.Ref_Attacking`))
  (bind _returnvalue (- (`self.K2_GetActorLocation` _ref_attacking) (`self.K2_GetActorLocation`)))
  ;[1 1 1] Bullet follow Enemy
  (`/Engine/EditorBlueprintResources/StandardMacros.IsValid` _ref_attacking
    (:`Is Valid`
      (`self.K2_AddActorWorldOffset` (* (/ _returnvalue (`KismetMathLibrary.VSize` _returnvalue)) (`self.speed`)) true))
    (:`Is Not Valid`
      (`self.K2_DestroyActor`))))

(event `self.Box.OnComponentBeginOverlap`
  (params (OverlappedComponent :type "PrimitiveComponent Object Reference") (OtherActor :type "Actor Object Reference") (OtherComp :type "PrimitiveComponent Object Reference") (OtherBodyIndex :type Integer) (bFromSweep :type Boolean) (SweepResult :type "HitResult Structure (by ref)"))
  (`self.Overlap` OtherActor))

(event `Overlap`
  (params (OverlapActor :type "Actor Object Reference")))

(fn `UserConstructionScript`)