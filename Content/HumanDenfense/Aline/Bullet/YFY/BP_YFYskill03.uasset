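; BP_YFYskill03 is a skill actor that deals repeating area damage, apparently fire, to targets around its spawn location.
; On BeginPlay it runs one multi-sphere object trace, with debug drawing on, and stores the hit actors in FireEnemy.
; A looping timer calls damageEveryEnemy, which applies damage to each still-valid stored actor.
; The target list is never refreshed, so actors keep taking damage regardless of later position.
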(event `self.ReceiveBeginPlay`
  (bind _location (`self.Location`))
  (bind _outhits (`KismetSystemLibrary.SphereTraceMultiForObjects` :`Start` _location :`End` _location :`Radius` (`self.EXPradius`) :`ObjectTypes` (`|MakeArray` "ObjectTypeQuery8" :!type "EObjectTypeQuery Enum") :`DrawDebugType` "ForDuration"))
  (for _array_element _outhits
    (`KismetArrayLibrary.Array_Add` (`self.FireEnemy`) (`.HitActor` (`GameplayStatics.BreakHitResult` _array_element))))
  (`KismetSystemLibrary.K2_SetTimer` null "damageEveryEnemy" (`self.DelayTime`) true))

(fn `damageEveryEnemy`
  (for _array_element (`self.FireEnemy`)
    (`/Engine/EditorBlueprintResources/StandardMacros.IsValid` _array_element
      (:`Is Valid`
        (`GameplayStatics.ApplyDamage` _array_element (`self.Damage`) null self))))
  (return))

(fn `UserConstructionScript`)