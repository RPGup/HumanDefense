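; BP_ExpUperBase is a damageable ally structure that periodically grants experience to nearby allies.
; On BeginPlay a sphere trace caches actors in range once, and a looping timer feeds EXP to humans, gold makers and buff actors among them.
; It has its own health and leveling, shown through a UI_Health widget.
; Star level caps its level and sets the EXP granted, while level-ups add max HP.
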(event `self.ReceiveBeginPlay`
  (`self.SearchAline`)
  (`self.Exp+`)
  (bind _returnvalue (`KismetSystemLibrary.K2_SetTimerDelegate` (delegate `Exp+`) (`self.Updelay`) true))
  (set `self.EXPupTimer` _returnvalue))

(event `SearchAline`
  (bind _returnvalue (`self.K2_GetActorLocation`))
  (bind _outhits (`KismetSystemLibrary.SphereTraceMultiForObjects` :`Start` _returnvalue :`End` _returnvalue :`Radius` (`self.SearchRadius`) :`ObjectTypes` (`|MakeArray` "ObjectTypeQuery7" :!type "EObjectTypeQuery Enum") :`DrawDebugType` "ForDuration"))
  (`KismetArrayLibrary.Array_Clear` (`self.Ref_SearchedAline`))
  (for _array_element _outhits
    (`KismetArrayLibrary.Array_Add` (`self.Ref_SearchedAline`) (`.HitActor` (`GameplayStatics.BreakHitResult` _array_element)))))

(event `Exp+`
  (bind _expupnum (`self.ExpUpNum`))
  (for _array_element (`self.Ref_SearchedAline`)
    (bind _asbp_human (cast `/Game/HumanDenfense/Aline/Attack/BP_Human` _array_element)
      (:`then`
        (`/Game/HumanDenfense/Aline/Attack/BP_Human.CaculateExp` _asbp_human _expupnum))
      (:`CastFailed`
        (bind _asbp_gold_maker_base (cast `/Game/HumanDenfense/Aline/GoldMaker/BP_GoldMakerBase` _array_element)
          (:`then`
            (`/Game/HumanDenfense/Aline/GoldMaker/BP_GoldMakerBase.CaculateExp` _asbp_gold_maker_base _expupnum))
          (:`CastFailed`
            (bind _asbp_buff (cast `/Game/HumanDenfense/Aline/Buff/BP_Buff` _array_element)
              (:`then`
                (`/Game/HumanDenfense/Aline/Buff/BP_Buff.CaculateExp` _asbp_buff _expupnum))
              (:`CastFailed`
                (bind _asbp_gold_maker_base_2 (cast `/Game/HumanDenfense/Aline/GoldMaker/BP_GoldMakerBase` _array_element))
                (`/Game/HumanDenfense/Aline/GoldMaker/BP_GoldMakerBase.CaculateExp` _asbp_gold_maker_base_2 _expupnum)))))))
    (`KismetSystemLibrary.PrintString` "EXPup")))

(event `Star+`
  (bind _returnvalue (+ (`self.StarLevel`) 1))
  (if (not (== (`self.StarLevel`) 5))
    (bind _asui_health (cast `/Game/HumanDenfense/UI/aLINE/UI_Health` (`WidgetComponent.GetUserWidgetObject` (`self.HPandEXP`))))
    (set `/Game/HumanDenfense/UI/aLINE/UI_Health.Star` _returnvalue _asui_health)
    (bind _output_get (set `self.StarLevel` _returnvalue))
    (switch `int` _output_get
      (:`1`
        (set `self.ExpUpNum` 5))
      (:`2`
        (set `self.ExpUpNum` 10))
      (:`3`
        (set `self.ExpUpNum` 20))
      (:`4`
        (set `self.ExpUpNum` 35))
      (:`5`
        (set `self.ExpUpNum` 70)))))

(event `LevelUP`
  (bind _asui_health (cast `/Game/HumanDenfense/UI/aLINE/UI_Health` (`WidgetComponent.GetUserWidgetObject` (`self.HPandEXP`))))
  (set `/Game/HumanDenfense/UI/aLINE/UI_Health.Level` (`self.Level`) _asui_health)
  (set `self.HP` (+ (`self.HP`) (`self.HPUP`)))
  (set `self.MaxHp` (+ (`self.HPUP`) (`self.MaxHp`))))

(event `self.ReceiveAnyDamage`
  (params (Damage :type "Float (single-precision)") (DamageType :type "DamageType Object Reference") (InstigatedBy :type "Controller Object Reference") (DamageCauser :type "Actor Object Reference"))
  (`self.CaculateHP` Damage))

(fn `CaculateEXP`
  (params (NewParam :type Integer))
  (bind _exp (`self.Exp`))
  (if (== (* (`self.StarLevel`) 10) (`self.Level`))
    (`KismetSystemLibrary.PrintString` "CanNotGetExp")
    (else
      (set `self.Exp` (+ NewParam (`self.Exp`)))
      (if (>= _exp (`self.LevelExp`)) :!label _label
        (set `self.Exp` (- _exp (`self.LevelExp`)))
        (set `self.Level` (+ (`self.Level`) 1))
        (`self.LevelUP`)
        (if (== (* (`self.StarLevel`) 10) (`self.Level`))
          (set `self.Exp` 0)
          (else
            (goto _label))))
      (bind _asui_health (cast `/Game/HumanDenfense/UI/aLINE/UI_Health` (`WidgetComponent.GetUserWidgetObject` (`self.HPandEXP`))))
      (`ProgressBar.SetPercent` (`/Game/HumanDenfense/UI/aLINE/UI_Health.ExpBar` _asui_health) (/ (`KismetMathLibrary.Conv_IntToDouble` (`self.Exp`)) (`KismetMathLibrary.Conv_IntToDouble` (`self.LevelExp`))))
      (return))))

(fn `CaculateHP`
  (params (A :type "Float (double-precision)"))
  (bind _maxhp (`self.MaxHp`))
  (bind _output_get (set `self.HP` (- (`self.HP`) A)))
  (bind _asui_health (cast `/Game/HumanDenfense/UI/aLINE/UI_Health` (`WidgetComponent.GetUserWidgetObject` (`self.HPANDEXP`))))
  (`ProgressBar.SetPercent` (`/Game/HumanDenfense/UI/aLINE/UI_Health.HealthBar` _asui_health) (/ _output_get (`self.MaxHp`)))
  (if (<= _output_get 0.0)
    (`self.K2_DestroyActor`)
    (`KismetSystemLibrary.PrintString` "death")
    (elif (>= (`self.HP`) _maxhp)
      (set `self.HP` _maxhp)))
  (return))

(fn `UserConstructionScript`)