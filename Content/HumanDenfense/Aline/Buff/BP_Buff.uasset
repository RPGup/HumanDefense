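; BP_Buff is a buff-giver actor with HP, armor, experience and levels, whose Buff event is an empty stub.
; On BeginPlay it caches BP_Base and sphere-traces within BuffRange for friendly actors, storing hits before calling Buff.
; That search runs before Wordlocation is assigned, so it uses the variable's prior value.
; CaculateExp raises Level at per-level thresholds, and LeverUp scales HP, armor and buff strength for levels two to five.
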(event `self.ReceiveBeginPlay`
  (bind _outactors (`GameplayStatics.GetAllActorsOfClass` "/Game/HumanDenfense/Aline/Base/BP_Base.BP_Base_C"))
  (set `self.Ref_Base` (`|GetArrayItem` _outactors))
  (`self.SearchFriend`)
  (set `self.wordlocation` (`self.K2_GetActorLocation`)))

(event `SearchFriend`
  (bind _ref_alinesearched (`self.Ref_AlineSearched`))
  (bind _wordlocation (`self.wordlocation`))
  (bind (_outhits _returnvalue) (`KismetSystemLibrary.SphereTraceMultiForObjects` :`Start` _wordlocation :`End` _wordlocation :`Radius` (`self.BuffRange`) :`ObjectTypes` (`|MakeArray` "ObjectTypeQuery7" :!type "EObjectTypeQuery Enum") :`DrawDebugType` "ForDuration"))
  (if _returnvalue
    (`KismetArrayLibrary.Array_Clear` _ref_alinesearched)
    (for _array_element _outhits
      (`KismetArrayLibrary.Array_Add` _ref_alinesearched (`.HitActor` (`GameplayStatics.BreakHitResult` _array_element))))
    (`self.Buff`)
    (`KismetSystemLibrary.PrintString` "Search compelet")))

(event `Buff`)

(fn `CaculateExp`
  (params (exp :type Integer))
  (bind _output (`|GetArrayItem` (`self.LevelExp`) (`self.Level`)))
  (bind _output_get (set `self.Exp` (+ exp (`self.Exp`))))
  (if (>= _output_get _output)
    (set `self.Exp` (- _output_get _output))
    (set `self.Level` (+ (`self.Level`) 1))
    (`self.LeverUp`))
  (return))

(fn `LeverUp`
  (bind _leverupscale (`self.LeverUpScale`))
  (switch `int` (`self.Level`)
    (:`Default`
      _)
    (:`0`
      _)
    (:`1`
      _)
    (:`2`
      (set `self.HP` (* (`self.HP`) _leverupscale) :!label _label)
      (set `self.Amor` (* (`self.Amor`) _leverupscale))
      (set `self.BuffUp` (* (`self.BuffUp`) _leverupscale)))
    (:`3`
      (goto _label))
    (:`4`
      (goto _label))
    (:`5`
      (goto _label)))
  (return))

(fn `UserConstructionScript`)