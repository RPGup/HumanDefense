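; BP_BuffAttack is an attack buff actor that periodically boosts the damage of allied humans.
; Its Buff event multiplies NomalDamage by BuffUp on each valid BP_Human in RefAlineSearched, waits BuffTime, divides it back, then waits BuffDelay and repeats indefinitely.
; The revert pass re-reads the array, so membership changes during the buff can leave damage values unbalanced.
; Nothing in this graph calls Buff or fills the array.
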(event `self.Buff`
  (for _array_element (`self.Ref_AlineSearched`) :!label _label
    (if (`KismetSystemLibrary.IsValid` _array_element)
      (bind _asbp_human (cast `/Game/HumanDenfense/Aline/Attack/BP_Human` _array_element))
      (set `/Game/HumanDenfense/Aline/Attack/BP_Human.NomalDamage` (* (`/Game/HumanDenfense/Aline/Attack/BP_Human.NomalDamage` _asbp_human) (`self.BuffUp`)) _asbp_human)
      (`KismetSystemLibrary.PrintString` "UP")))
  (`KismetSystemLibrary.Delay` (`self.BuffTime`))
  (for _array_element_2 (`self.Ref_AlineSearched`)
    (if (`KismetSystemLibrary.IsValid` _array_element_2)
      (bind _asbp_human_2 (cast `/Game/HumanDenfense/Aline/Attack/BP_Human` _array_element_2))
      (set `/Game/HumanDenfense/Aline/Attack/BP_Human.NomalDamage` (/ (`/Game/HumanDenfense/Aline/Attack/BP_Human.NomalDamage` _asbp_human_2) (`self.BuffUp`)) _asbp_human_2)
      (`KismetSystemLibrary.PrintString` "DOWN")))
  (`KismetSystemLibrary.Delay` (`self.BuffDelay`))
  (goto _label))

(fn `UserConstructionScript`
  (`parent.UserConstructionScript`))