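; BP_JS is a melee ("JinZhan") Aline attack unit whose montage notifies deal damage to its target or to an area.
; Attackto hits the first enemy normally, or, when the timer-driven Skill01 is ready, capsule-traces for double damage with an IsTwice-toggled delayed repeat.
; Skill02 raises damage, adding life steal (HPjiqu) at level 30, and Skill03 halves attack and skill delays.
; Skill01Body holds a separate single-pass area attack, uncalled in this file.
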(event `self.Skill02`
  (if (== (`self.Level`) 30)
    (set `self.NomalDamage` (* (`self.NomalDamage`) 1.3))
    (set `self.HPjiqu` 0.3)
    (else
      (set `self.NomalDamage` (+ (* (`self.DamageUP`) 0.3) (`self.NomalDamage`)))
      (set `self.DamageUP` (* (`self.DamageUP`) 1.3)))))

(event `self.Skill03`
  (set `self.AttackDelay` (* (`self.AttackDelay`) 0.5))
  (set `self.Skill01Delay` (* (`self.Skill01Delay`) 0.5)))

(event `self.AttackTo`
  (bind _wordlocation (`self.wordlocation`))
  ;[1 1 1] NormalAttackAndSkill01
  (if (`self.Skill01Ready?`)
    (`|PlayMontage` (`self.Mesh`) (`self.Ref_Montage`) 1.0 0.0 (`self.StartSection`)
      (:`then`
        (set `self.isAttacking` true))
      (:`OnCompleted`
        (set `self.isAttacking` false))
      (:`OnNotifyBegin`
        (bind _outhits (`KismetSystemLibrary.CapsuleTraceMultiForObjects` :`Start` _wordlocation :`End` _wordlocation :`Radius` (`self.SkillRadius`) :`HalfHeight` (`self.SkillHalfHeight`) :`ObjectTypes` (`|MakeArray` "ObjectTypeQuery8" :!type "EObjectTypeQuery Enum") :`DrawDebugType` "ForDuration"))
        (`KismetArrayLibrary.Array_Clear` (`self.Skill01Searched`))
        (for _array_element _outhits
          (`KismetArrayLibrary.Array_Add` (`self.Skill01Searched`) (`.HitActor` (`GameplayStatics.BreakHitResult` _array_element))))
        (for _array_element_2 (`self.Skill01Searched`) :!label _label
          (`/Engine/EditorBlueprintResources/StandardMacros.IsValid` _array_element_2
            (:`Is Valid`
              (`GameplayStatics.ApplyDamage` _array_element_2 (* (`self.NomalDamage`) 2.0) null self)
              (set `self.IsTwice` (not (`self.IsTwice`)))
              (if (`self.IsTwice`)
                (set `self.Skill01Ready?` false)
                (`KismetSystemLibrary.K2_ClearAndInvalidateTimerHandle` (`self.Skill01Timer`))
                (bind _returnvalue (`KismetSystemLibrary.K2_SetTimerDelegate` (delegate `SkillReset`) (`self.Skill01Delay`) true))
                (set `self.Skill01Timer` _returnvalue)
                (else
                  (`KismetSystemLibrary.Delay` 0.1)
                  (goto _label))))))))
    (else
      (`|PlayMontage` (`self.Mesh`) (`self.Ref_Montage`) 1.0 0.0 (`self.StartSection`)
        (:`then`
          (set `self.isAttacking` true))
        (:`OnCompleted`
          (set `self.isAttacking` false))
        (:`OnNotifyBegin`
          (`GameplayStatics.ApplyDamage` (`self.Ref_FirstEnemy`) (`self.NomalDamage`) null self))))))

(event `self.Skill01`
  (bind _returnvalue (`KismetSystemLibrary.K2_SetTimerDelegate` (delegate `SkillReset`) (`self.Skill01Delay`) true))
  (set `self.Skill01Timer` _returnvalue))

(event `SkillReset`
  (set `self.Skill01Ready?` true))

(fn `Skill01Body`
  (bind _wordlocation (`self.wordlocation`))
  (bind (_outhits _returnvalue) (`KismetSystemLibrary.CapsuleTraceMultiForObjects` :`Start` _wordlocation :`End` _wordlocation :`Radius` (`self.SkillRadius`) :`HalfHeight` (`self.SkillHalfHeight`) :`ObjectTypes` (`|MakeArray` "ObjectTypeQuery8" :!type "EObjectTypeQuery Enum") :`DrawDebugType` "ForDuration"))
  (if _returnvalue
    ;[1 1 1] NeedXIUGAI   NeedAnime
    (`self.PlayAnimMontage` "/Game/Mannequin/Animations/Aline_Montage.Aline_Montage" 1.0 "attack")
    (for _array_element _outhits
      (bind (_bblockinghit _binitialoverlap _time _distance _location _impactpoint _normal _impactnormal _physmat _hitactor) (`GameplayStatics.BreakHitResult` _array_element))
      (`/Engine/EditorBlueprintResources/StandardMacros.IsValid` _hitactor
        (:`Is Valid`
          (`GameplayStatics.ApplyDamage` _hitactor (* (`self.NomalDamage`) 2.0) null self))))
    (return)))

(fn `UserConstructionScript`
  (`parent.UserConstructionScript`))