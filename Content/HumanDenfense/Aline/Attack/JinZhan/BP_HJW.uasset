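; BP_HJW is a melee (JinZhan) unit Blueprint with two skills, apparently an armor boost and a taunt.
; Skill01 sets Amor to a fixed value.
; Skill02 starts a looping timer that sphere-traces around Wordlocation and casts hits to BP_Enemy.
; The taunt is only a stub: it prints "Chaofeng" for an enemy and returns, and nothing here clears the timer or uses Skill02Time.
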(event `self.ReceiveBeginPlay`
  (`parent.ReceiveBeginPlay`))

(event `self.Skill01`
  (set `self.Amor` 1.0))

(event `self.Skill02`
  (bind _returnvalue (`KismetSystemLibrary.K2_SetTimer` self "Skill02Body" (`self.Skill02Delay`) true))
  (set `self.Skill02Timer` _returnvalue))

(fn `Skill02Body`
  (bind _wordlocation (`self.wordlocation`))
  (bind (_outhits _returnvalue) (`KismetSystemLibrary.SphereTraceMultiForObjects` :`Start` _wordlocation :`End` _wordlocation :`Radius` (`self.Skill02Range`) :`ObjectTypes` (`|MakeArray` "ObjectTypeQuery8" :!type "EObjectTypeQuery Enum") :`DrawDebugType` "ForDuration"))
  (if _returnvalue
    (for _array_element _outhits
      (cast `/Game/HumanDenfense/Enemy/BP_Enemy` (`.HitActor` (`GameplayStatics.BreakHitResult` _array_element)))
      (`KismetSystemLibrary.PrintString` "Chaofeng")
      (return))))

(fn `UserConstructionScript`
  (`parent.UserConstructionScript`))