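; Base human defender tower that searches for enemies and attacks the one nearest the player's base (BP_Base).
; A delayed Search loop sphere-traces attack range, or move range first when CanMove is set, and FindFirstEnemy picks the target.
; AttackNormal faces the target and repeats a montage while it stays in range, calling AttackTo on notifies.
; AttackTo is empty here, and MoveTo's AIMoveTo has no destination wired.
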(event `self.ReceiveBeginPlay`
  (bind _outactors (`GameplayStatics.GetAllActorsOfClass` "/Game/HumanDenfense/Aline/Base/BP_Base.BP_Base_C"))
  (set `self.Ref_Base` (`|GetArrayItem` _outactors))
  (`self.Search`))

(event `Search`
  (bind _returnvalue (`self.K2_GetActorLocation`))
  (bind _returnvalue_2 (`self.K2_GetActorLocation`))
  (`KismetSystemLibrary.Delay` (`self.AtackDelay`))
  (if (`self.CanMove`)
    (bind (_outhits _returnvalue_3) (`KismetSystemLibrary.SphereTraceMultiForObjects` :`Start` _returnvalue :`End` _returnvalue :`Radius` (`self.MoveRange`) :`ObjectTypes` (`|MakeArray` "ObjectTypeQuery8" :!type "EObjectTypeQuery Enum") :`DrawDebugType` "ForDuration"))
    (if _returnvalue_3
      (`KismetArrayLibrary.Array_Clear` (`self.Ref_SearchedEnemyMove`))
      (for _array_element _
        (`KismetArrayLibrary.Array_Add` (`self.Ref_SearchedEnemy`) (`.HitActor` (`GameplayStatics.BreakHitResult` _array_element))))
      (if (> (`KismetArrayLibrary.Array_Length` (`self.Ref_SearchedEnemy`)) 0)
        (bind _issearched_ (`self.FindFirstEnemy`))
        (if _issearched_
          (`self.MoveTo`)))
      (`self.Search`)
      (else
        (bind (_outhits_2 _returnvalue_4) (`KismetSystemLibrary.SphereTraceMultiForObjects` :`Start` _returnvalue_2 :`End` _returnvalue_2 :`Radius` (`self.AttackRange`) :`ObjectTypes` (`|MakeArray` "ObjectTypeQuery8" :!type "EObjectTypeQuery Enum") :`DrawDebugType` "ForDuration" :!label _label))
        (if _returnvalue_4
          (`KismetArrayLibrary.Array_Clear` (`self.Ref_SearchedEnemy`))
          (for _array_element_2 _outhits_2
            (`KismetArrayLibrary.Array_Add` (`self.Ref_SearchedEnemy`) (`.HitActor` (`GameplayStatics.BreakHitResult` _array_element_2))))
          (if (> (`KismetArrayLibrary.Array_Length` (`self.Ref_SearchedEnemy`)) 0)
            (bind _issearched__2 (`self.FindFirstEnemy`))
            (if _issearched__2
              (`self.AttackNormal`)
              (else
                (`self.Search` :!label _label_2)))
            (else
              (goto _label_2)))
          (else
            (goto _label_2)))))
    (else
      (goto _label))))

(event `AttackNormal`
  (bind _ref_firstenemy (`self.Ref_FirstEnemy`))
  (bind (_returnvalue_roll _returnvalue_pitch _returnvalue_yaw) (`KismetMathLibrary.BreakRotator` (`KismetMathLibrary.FindLookAtRotation` (`self.K2_GetActorLocation`) (`self.K2_GetActorLocation` (`self.Ref_FirstEnemy`)))))
  (`self.K2_SetActorRotation` (`KismetMathLibrary.MakeRotator` 0.0 0.0 _returnvalue_yaw))
  (`|PlayMontage` (`self.Aline`) (`self.Ref_Montage`) 1.0 0.0 (`self.StartSection`)
    (:`then`
      (set `self.isAttacking` true))
    (:`OnCompleted`
      (`KismetSystemLibrary.Delay` (`self.AtackDelay`))
      (if (`KismetSystemLibrary.IsValid` _ref_firstenemy)
        (if (> (`KismetMathLibrary.VSize` (- (`self.K2_GetActorLocation` _ref_firstenemy) (`self.K2_GetActorLocation` self))) (`self.AttackRange`))
          (`self.Search` :!label _label_3)
          (set `self.isAttacking` false)
          (else
            (`self.AttackNormal`)))
        (else
          (goto _label_3))))
    (:`OnNotifyBegin`
      (`self.AttackTo`))))

(event `AttackTo`)

(event `MoveTo`
  (`|AIMoveTo` null (0.0 0.0 0.0) null))

(fn `FindFirstEnemy`
  (returns (`IsSearched?` :type Boolean))
  (locals (Destance :type "Float (double-precision)" :default 999999.0))
  (for _array_element (`self.Ref_SearchedEnemy`)
    (bind _returnvalue (`KismetMathLibrary.VSize` (- (`self.K2_GetActorLocation` _array_element) (`self.K2_GetActorLocation` (`self.Ref_Base`)))))
    (if (<= _returnvalue (`local.Destance`))
      (set `local.Destance` _returnvalue)
      (set `self.Ref_FirstEnemy` _array_element)))
  (return (`KismetSystemLibrary.IsValid` (`self.Ref_FirstEnemy`))))

(fn `UserConstructionScript`)