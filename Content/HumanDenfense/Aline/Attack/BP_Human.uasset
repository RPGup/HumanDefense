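; BP_Human is a defender unit that automatically finds and attacks enemies, favoring those nearest BP_Base.
; A delayed Search loop sphere-traces for targets: mobile units chase within MoveRange of their spawn point and run back there, while stationary units attack within AttackRange.
; Attack montage notifies call AttackTo, an empty event here.
; It also defines experience and level-up functions that scale HP, armor and damage.
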(event `self.ReceiveBeginPlay`
  (bind _outactors (`GameplayStatics.GetAllActorsOfClass` "/Game/HumanDenfense/Aline/Base/BP_Base.BP_Base_C"))
  (set `self.Ref_Base` (`|GetArrayItem` _outactors))
  (`self.Search`)
  (set `self.wordlocation` (`self.K2_GetActorLocation`)))

(event `Search`
  (bind _returnvalue (`self.K2_GetActorLocation`))
  (bind _wordlocation (`self.wordlocation`))
  (bind _ref_searchedenemy (`self.Ref_SearchedEnemy`))
  (`KismetSystemLibrary.Delay` (`self.AtackDelay`))
  (if (`self.CanMove`)
    (if (and (not (`self.isbacking?`)) (`self.IsNotMoving`))
      (bind (_outhits _returnvalue_2) (`KismetSystemLibrary.SphereTraceMultiForObjects` :`Start` _wordlocation :`End` _wordlocation :`Radius` (`self.MoveRange`) :`ObjectTypes` (`|MakeArray` "ObjectTypeQuery8" :!type "EObjectTypeQuery Enum") :`DrawDebugType` "ForDuration"))
      (if _returnvalue_2
        (`KismetArrayLibrary.Array_Clear` (`self.Ref_SearchedEnemy`))
        (for _array_element _outhits
          (`KismetArrayLibrary.Array_Add` _ref_searchedenemy (`.HitActor` (`GameplayStatics.BreakHitResult` _array_element)))
          (`KismetSystemLibrary.PrintString` (`KismetStringLibrary.Conv_IntToString` (`KismetArrayLibrary.Array_Length` _ref_searchedenemy))))
        (if (> (`KismetArrayLibrary.Array_Length` (`self.Ref_SearchedEnemy`)) 0)
          (bind _issearched (`self.FindFirstEnemy`))
          (if _issearched
            (if (> (`KismetMathLibrary.VSize` (- (`self.K2_GetActorLocation`) (`self.wordlocation`))) (`self.MoveRange`))
              (`self.Back`)
              (else
                (`self.MoveTo`)
                (`KismetSystemLibrary.PrintString` "Move")))
            (else
              (`self.Search` :!label _label)))
          (else
            (goto _label)))
        (else
          (`self.Back`)))
      (else
        (`KismetSystemLibrary.PrintString` "Hello")))
    (else
      (bind (_outhits_2 _returnvalue_3) (`KismetSystemLibrary.SphereTraceMultiForObjects` :`Start` _returnvalue :`End` _returnvalue :`Radius` (`self.AttackRange`) :`ObjectTypes` (`|MakeArray` "ObjectTypeQuery8" :!type "EObjectTypeQuery Enum") :`DrawDebugType` "ForDuration"))
      (if _returnvalue_3
        (`KismetArrayLibrary.Array_Clear` (`self.Ref_SearchedEnemy`))
        (for _array_element_2 _outhits_2
          (`KismetArrayLibrary.Array_Add` (`self.Ref_SearchedEnemy`) (`.HitActor` (`GameplayStatics.BreakHitResult` _array_element_2))))
        (if (> (`KismetArrayLibrary.Array_Length` (`self.Ref_SearchedEnemy`)) 0)
          (bind _issearched_2 (`self.FindFirstEnemy`))
          (if _issearched_2
            (`self.AttackNormal`)
            (else
              (`self.Search` :!label _label_2)))
          (else
            (goto _label_2)))
        (else
          (`self.Search`))))))

(event `AttackNormal`
  (bind _ref_firstenemy (`self.Ref_FirstEnemy`))
  (bind (_returnvalue_roll _returnvalue_pitch _returnvalue_yaw) (`KismetMathLibrary.BreakRotator` (`KismetMathLibrary.FindLookAtRotation` (`self.K2_GetActorLocation`) (`self.K2_GetActorLocation` (`self.Ref_FirstEnemy`)))))
  (`self.K2_SetActorRotation` (`KismetMathLibrary.MakeRotator` 0.0 0.0 _returnvalue_yaw))
  (`|PlayMontage` (`self.Mesh`) (`self.Ref_Montage`) 1.0 0.0 (`self.StartSection`)
    (:`then`
      (set `self.isAttacking` true))
    (:`OnCompleted`
      (`KismetSystemLibrary.Delay` (`self.AtackDelay`))
      (if (`KismetSystemLibrary.IsValid` _ref_firstenemy)
        (if (> (`KismetMathLibrary.VSize` (- (`self.K2_GetActorLocation` _ref_firstenemy) (`self.K2_GetActorLocation` self))) (`self.AttackRange`))
          (`self.Search` :!label _label_3)
          (set `self.isAttacking` false)
          (else
            (`self.AttackNormal`)))
        (else
          (goto _label_3))))
    (:`OnNotifyBegin`
      (`self.AttackTo`))))

(event `AttackTo`)

(event `MoveTo`
  (set `self.IsNotMoving` false)
  (`|AIMoveTo` self (0.0 0.0 0.0) (`self.Ref_FirstEnemy`) (`self.AttackRange`)
    (:`OnSuccess`
      _)
    (:`OnFail`
      _))
  (set `self.IsNotMoving` true)
  (`|PlayMontage` (`self.Mesh`) (`self.Ref_Montage`) 1.0 0.0 (`self.StartSection`)
    (:`then`
      (set `self.isAttacking` true))
    (:`OnCompleted`
      (set `self.isAttacking` false)
      (`self.Search`))
    (:`OnNotifyBegin`
      (`self.AttackTo`))))

(event `Back`
  (if (== (`self.K2_GetActorLocation`) (`self.wordlocation`) :`ErrorTolerance` 0.01)
    (`self.Search` :!label _label_4)
    (else
      (set `CharacterMovementComponent.MaxWalkSpeed` 1500.0 (`self.CharacterMovement`))
      (`|AIMoveTo` self (`self.wordlocation`) null 0.0
        (:`then`
          (set `self.isbacking?` true))
        (:`OnSuccess`
          (set `CharacterMovementComponent.MaxWalkSpeed` (`self.MaxWalkSP`) (`self.CharacterMovement`) :!label _label_5)
          (set `self.isbacking?` false)
          (goto _label_4))
        (:`OnFail`
          (goto _label_5))))))

(fn `CaculateExp`
  (params (Exp :type Integer))
  (bind _output (`|GetArrayItem` (`self.LevelExp`) (`self.Level`)))
  (bind _output_get (set `self.Exp` (+ Exp (`self.Exp`))))
  (if (>= _output_get _output)
    (set `self.Exp` (- _output_get _output))
    (set `self.Level` (+ (`self.Level`) 1))
    (`self.LevelUp`))
  (return))

(fn `FindFirstEnemy`
  (returns (IsSearched :type Boolean))
  (locals (Destance :type "Float (double-precision)" :default 9999.0))
  (for _array_element (`self.Ref_SearchedEnemy`)
    (if (`KismetSystemLibrary.IsValid` _array_element)
      (bind _returnvalue (`KismetMathLibrary.VSize` (- (`self.K2_GetActorLocation` _array_element) (`self.K2_GetActorLocation` (`self.Ref_Base`)))))
      (if (<= _returnvalue (`local.Destance`))
        (set `local.Destance` _returnvalue)
        (set `self.Ref_FirstEnemy` _array_element))))
  (return (`KismetSystemLibrary.IsValid` (`self.Ref_FirstEnemy`))))

(fn `LevelUp`
  (bind _levelupscale (`self.LevelUpScale`))
  (switch `int` (`self.Level`)
    (:`Default`
      _)
    (:`0`
      _)
    (:`1`
      _)
    (:`2`
      (set `self.HP` (* (`self.HP`) _levelupscale) :!label _label)
      (set `self.Amor` (* (`self.Amor`) _levelupscale))
      (set `self.NomalDamage` (* (`self.NomalDamage`) _levelupscale)))
    (:`3`
      (goto _label))
    (:`4`
      (goto _label))
    (:`5`
      (goto _label)))
  (return))

(fn `UserConstructionScript`
  (set `CharacterMovementComponent.MaxWalkSpeed` (`self.MaxWalkSP`) (`self.CharacterMovement`)))