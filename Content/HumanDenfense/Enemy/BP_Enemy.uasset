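; BP_Enemy is an enemy that heads for the first BP_Base actor in the level using AI MoveTo on spawn.
; Any damage is reduced by armor, clamped, and subtracted from HP, updating the health bar widget; the enemy is destroyed at zero HP.
; FucAlineSearch box-traces forward over the attack range with debug drawing, but nothing here calls it or uses its result.
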(event `self.ReceiveBeginPlay`
  (bind _outactors (`GameplayStatics.GetAllActorsOfClass` "/Game/HumanDenfense/Aline/Base/BP_Base.BP_Base_C"))
  (`|AIMoveTo` self (0.0 0.0 0.0) (`|GetArrayItem` _outactors) 50.0))

(event `self.ReceiveAnyDamage`
  (params (Damage :type "Float (single-precision)") (DamageType :type "DamageType Object Reference") (InstigatedBy :type "Controller Object Reference") (DamageCauser :type "Actor Object Reference"))
  (bind _hp (`self.HP`))
  (bind _output_get (set `self.HP` (- (`self.HP`) (`KismetMathLibrary.FClamp` (- Damage (`self.amor`)) 0.1 10.0))))
  (`KismetSystemLibrary.PrintString` (`KismetStringLibrary.Conv_DoubleToString` _output_get))
  (bind _asui_heath_bar (cast `/Game/HumanDenfense/UI/UI_HeathBar` (`WidgetComponent.GetUserWidgetObject` (`self.Health`))))
  (set `/Game/HumanDenfense/UI/UI_HeathBar.HP` (/ _hp (`self.MaxHP`)) _asui_heath_bar)
  (if (<= _hp 0.0)
    (`KismetSystemLibrary.PrintString` "Death")
    (`self.K2_DestroyActor`)))

(fn `Fuc_AlineSearch`
  (bind _returnvalue (`self.K2_GetActorLocation`))
  (`KismetSystemLibrary.BoxTraceSingleForObjects` :`Start` _returnvalue :`End` (+ (* (`KismetMathLibrary.GetForwardVector` (`self.K2_GetActorRotation`)) (`self.AttackRange`)) _returnvalue) :`HalfSize` (50.0 50.0 50.0) :`ObjectTypes` (`|MakeArray` "ObjectTypeQuery7" :!type "EObjectTypeQuery Enum") :`DrawDebugType` "ForDuration"))

(fn `UserConstructionScript`)