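; BP_C is an enemy Blueprint in HumanDenfense whose skill is an area attack that damages and stuns humans.
; SkillBody runs a multi-sphere object trace of SkillRange radius at the location of the RefSearchedAline actor, with timed debug drawing.
; Each hit that casts to BP_Human receives XuanYun (stun) with the attack damage and stun time, though the first failed cast stops the event.
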(event `self.SkillBody`
  (bind _returnvalue (`self.K2_GetActorLocation` (`self.Ref_SearchedAline`)))
  (bind _outhits (`KismetSystemLibrary.SphereTraceMultiForObjects` :`Start` _returnvalue :`End` _returnvalue :`Radius` (`self.SkillRange`) :`ObjectTypes` (`|MakeArray` "ObjectTypeQuery7" :!type "EObjectTypeQuery Enum") :`DrawDebugType` "ForDuration"))
  (for _array_element _outhits
    (bind _asbp_human (cast `/Game/HumanDenfense/Aline/Attack/BP_Human` (`.HitActor` (`GameplayStatics.BreakHitResult` _array_element))))
    (`/Game/HumanDenfense/Aline/Attack/BP_Human.XuanYun` _asbp_human (`self.AttackDamage`) (`self.XuanYuntime`))))

(fn `UserConstructionScript`
  (`parent.UserConstructionScript`))