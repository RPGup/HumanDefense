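; Touch-controlled camera pawn that registers with BP_PlayerContol and forwards touch press, move and release to it and the UTC touch components.
; First-finger swipes pan the pawn in world X/Y, except while the controller is building or a pinch is active.
; Pinching compares finger distance to its starting value to step the spring arm length within fixed limits.
; MoveScream nudges a stored screen point and deprojects it to position Cube; its clamped actor-move code is unconnected.
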(event `self.ReceiveBeginPlay`
  (bind _asbp_player_contol (cast `/Game/HumanDenfense/BluePrint/BP_PlayerContol` (`GameplayStatics.GetPlayerController` 0)))
  (set `self.control` _asbp_player_contol)
  (set `/Game/HumanDenfense/BluePrint/BP_PlayerContol.CameraPawn` self _asbp_player_contol)
  (set `self.Location` (`self.K2_GetActorLocation`)))

(event `self.UTCSwipeToMoveComponent.On Delta X Changed`
  (params (Value :type "Float (single-precision)"))
  (if (`self.IsSuofang`)
    _
    (elif (and (not (`/Game/HumanDenfense/BluePrint/BP_PlayerContol.IsBuilding` (`self.control`))) (`|EnumEquality` (stale `InputTouch` FingerIndex) "Touch1"))
      (`self.K2_AddActorWorldOffset` (`KismetMathLibrary.MakeVector` (* Value -10.0))))))

(event `self.UTCSwipeToMoveComponent.On Delta Y Changed`
  (params (Value :type "Float (single-precision)"))
  (if (`self.IsSuofang`)
    _
    (elif (and (not (`/Game/HumanDenfense/BluePrint/BP_PlayerContol.IsBuilding` (`self.control`))) (`|EnumEquality` (stale `InputTouch` FingerIndex) "Touch1"))
      (`self.K2_AddActorWorldOffset` (`KismetMathLibrary.MakeVector` 0.0 (* Value -10.0))))))

(event `InputTouch`
  (params (Location :type "Vector Structure") (FingerIndex :type "ETouchIndex Enum"))
  (bind _control (`self.control`))
  (:`Pressed`
    (`/Game/HumanDenfense/BluePrint/BP_PlayerContol.Pressed` _control)
    (set `self.IF_Touch1OrTouch` true)
    (`/Game/UltimateTouchComponents/Core/UTCMacroLibrary.UTC Touch Input Manager` Location FingerIndex :!label _label))
  (:`Released`
    (`/Game/HumanDenfense/BluePrint/BP_PlayerContol.Released` _control FingerIndex)
    (set `self.IF_Touch1OrTouch` false)
    (bind _utc_component (`/Game/UltimateTouchComponents/Core/UTCMacroLibrary.UTC Is Finger Location Exists` (`self.K2_GetComponentsByClass` "/Game/UltimateTouchComponents/Core/UTCComponent.UTCComponent_C") FingerIndex)
      (:`True`
        (`/Game/UltimateTouchComponents/Core/UTCComponent.On Event Touch Released` _utc_component Location FingerIndex))))
  (:`Moved`
    (`/Game/HumanDenfense/BluePrint/BP_PlayerContol.Move` _control FingerIndex)
    (goto _label :!via `Moved`)))

(event `self.UTCPinchComponent.On Two Fingers Pressed`
  (params (`Pan Location` :type "Vector Structure"))
  (bind _control (`self.control`))
  (bind (_locationx _locationy) (`PlayerController.GetInputTouchState` _control "Touch1"))
  (bind (_locationx_2 _locationy_2) (`PlayerController.GetInputTouchState` _control "Touch2"))
  (set `self.IsSuofang` true)
  (set `self.StartDestance` (`KismetMathLibrary.VSize2D` (- (`KismetMathLibrary.MakeVector2D` _locationx _locationy) (`KismetMathLibrary.MakeVector2D` _locationx_2 _locationy_2)))))

(event `self.UTCPinchComponent.On Two Fingers Move`
  (params (Zoom :type "Float (single-precision)") (`Rotation Angle` :type "Float (single-precision)") (`Initial Pan Location` :type "Vector Structure") (`Current Pan Location` :type "Vector Structure") (`Pan Offset` :type "Vector Structure"))
  (bind _control (`self.control`))
  (bind _springarm (`self.SpringArm`))
  (bind _springarm_2 (`self.SpringArm`))
  (bind _startdestance (`self.StartDestance`))
  (bind _enddestance (`self.EndDestance`))
  (bind _enddestance_2 (`self.EndDestance`))
  (bind _startdestance_2 (`self.StartDestance`))
  (bind (_locationx _locationy) (`PlayerController.GetInputTouchState` _control "Touch2"))
  (bind (_locationx_2 _locationy_2) (`PlayerController.GetInputTouchState` _control "Touch1"))
  (bind _returnvalue (+ (`SpringArmComponent.TargetArmLength` _springarm) 20.0))
  (bind _returnvalue_2 (+ (`SpringArmComponent.TargetArmLength` _springarm_2) -20.0))
  ;[1 1 1] suofang
  (if (`|EnumEquality` (stale `InputTouch` FingerIndex) "Touch2")
    (set `self.EndDestance` (`KismetMathLibrary.VSize2D` (- (`KismetMathLibrary.MakeVector2D` _locationx_2 _locationy_2) (`KismetMathLibrary.MakeVector2D` _locationx _locationy))))
    (if (`self.IF_Touch1OrTouch`)
      (`KismetSystemLibrary.PrintString` (`KismetStringLibrary.Concat_StrStr` (`KismetStringLibrary.Conv_DoubleToString` _startdestance) "   bi    " (`KismetStringLibrary.Conv_DoubleToString` _enddestance)) true true (struct :`R` 1.0 :`B` 0.980678 :`A` 1.0))
      (if (< _startdestance _enddestance)
        (`/Engine/EditorBlueprintResources/StandardMacros.CompareFloat` _returnvalue_2 200.0
          (:`>`
            (set `SpringArmComponent.TargetArmLength` _returnvalue_2 _springarm_2)))
        (else
          (`KismetSystemLibrary.PrintString` (`KismetStringLibrary.Concat_StrStr` (`KismetStringLibrary.Conv_DoubleToString` _startdestance_2) "  bi   " (`KismetStringLibrary.Conv_DoubleToString` _enddestance_2)) true true (struct :`R` 1.0 :`B` 0.980678 :`A` 1.0))
          (if (> _startdestance_2 _enddestance_2)
            (`/Engine/EditorBlueprintResources/StandardMacros.CompareFloat` _returnvalue 2000.0
              (:`<`
                (set `SpringArmComponent.TargetArmLength` _returnvalue _springarm)))
            (else
              (`KismetSystemLibrary.PrintString` "Hello" true true (struct :`R` 1.0 :`G` 0.146695 :`A` 1.0)))))))))

(event `self.UTCPinchComponent.On Two Fingers Released`
  (params (Zoom :type "Float (single-precision)") (`Rotation Angle` :type "Float (single-precision)") (`Initial Pan Location` :type "Vector Structure") (`Current Pan Location` :type "Vector Structure") (`Pan Offset` :type "Vector Structure"))
  ;[1 1 1] suofang
  (set `self.IsSuofang` false))

(fn `MoveScream`
  (params (InVec :type "Vector2D Structure"))
  (locals (X :type "Float (double-precision)" :default 0.0) (Y :type "Float (double-precision)" :default 0.0))
  (bind (_x _y) (`KismetMathLibrary.BreakVector2D` InVec))
  (bind (_x_2 _y_2) (`KismetMathLibrary.BreakVector2D` (`self.CameraScreenLocation`)))
  (if (> _x _x_2)
    (set `local.X` (+ _x 1.0))
    (else
      (set `local.X` (- _x 1.0))))
  (if (> _y _y_2)
    (set `local.Y` (+ _y 10.0))
    (else
      (set `local.Y` (- _y 10.0))))
  (bind _output_get (set `self.CameraScreenLocation` (`KismetMathLibrary.MakeVector2D` (`local.X`) (`local.Y`))))
  (`SceneComponent.K2_SetWorldLocation` (`self.Cube`) (`KismetMathLibrary.MakeVector` (.x (`GameplayStatics.DeprojectScreenToWorld` (`self.control`) _output_get)) (.y (`GameplayStatics.DeprojectScreenToWorld` (`self.control`) _output_get)) 300.0) false false)
  (return))

(fn `SetPosition`
  (params (CameraScreenLocation1 :type "Vector2D Structure"))
  (set `self.CameraScreenLocation` CameraScreenLocation1)
  (return))

(fn `UserConstructionScript`)