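; Player controller for a human-defense game, handling random card draws and touch drag-and-drop placement of units.
; On BeginPlay it creates the main UI, caches the base and spawns a hidden drag preview actor.
; FucSelect spends base gold on a random card with weighted star tiers, and FucBuild applies its mesh to the preview.
; While building, touch traces move the preview; release spawns the card's class and copies its level and stars.
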(event `self.ReceiveBeginPlay`
  (bind _returnvalue (`|CreateWidget` "/Game/HumanDenfense/UI/Main.Main_C"))
  (set `self.Main` _returnvalue)
  (`UserWidget.AddToViewport` _returnvalue 0)
  (bind _outactors (`GameplayStatics.GetAllActorsOfClass` "/Game/HumanDenfense/BluePrint/Aline/Base/BP_Base.BP_Base_C"))
  (set `self.Base` (`|GetArrayItem` _outactors))
  (bind _returnvalue_2 (`|SpawnActorFromClass` "/Game/HumanDenfense/BluePrint/BP_DragSlot.BP_DragSlot_C" (`KismetMathLibrary.MakeTransform` (0.0 0.0 -300.0) (struct) (1.0 1.0 1.0)) "Undefined" "OverrideRootScale" null null))
  (set `self.DragRef` _returnvalue_2)
  (`WidgetBlueprintLibrary.SetInputMode_GameAndUIEx` self null))

(event `Key|LeftMouseButton`
  (params (Key :type "Key Structure")))

(event `InputTouch`
  (params (Location :type "Vector Structure") (FingerIndex :type "ETouchIndex Enum"))
  (bind (_locationx _locationy) (`self.GetInputTouchState` FingerIndex))
  (bind (_locationx_2 _locationy_2) (`self.GetInputTouchState` FingerIndex))
  (bind (_jg_alinebuild_image _jg_alinebuild_classref _jg_alinebuild_level _jg_alinebuild_starlevel) (break `/Game/HumanDenfense/BluePrint/JG_PAI` (`self.JG_AlineBuild`)))
  (bind (_worldlocation _worlddirection) (`self.DeprojectScreenPositionToWorld` _locationx_2 _locationy_2))
  (bind (_worldlocation_2 _worlddirection_2) (`self.DeprojectScreenPositionToWorld` _locationx _locationy))
  ;[1 1 1] Touch Event
  (:`Pressed`
    (if (`self.IsBuilding`)
      (set `self.CanMove` true)))
  (:`Released`
    (if (`self.IsBuilding`)
      (set `self.CanMove` false)
      (`self.K2_SetActorLocation` (`self.DragRef`) (0.0 0.0 -500.0) false false)
      (bind (_outhit _returnvalue) (`KismetSystemLibrary.LineTraceSingleForObjects` :`Start` _worldlocation :`End` (+ (* _worlddirection 4000.0) _worldlocation) :`ObjectTypes` (`|MakeArray` "ObjectTypeQuery1" :!type "EObjectTypeQuery Enum") :`DrawDebugType` "ForDuration"))
      (if _returnvalue
        (bind _returnvalue_2 (`|SpawnActorFromClass` _jg_alinebuild_classref (`KismetMathLibrary.MakeTransform` (`.Location` (`GameplayStatics.BreakHitResult` _outhit))) "Undefined" "OverrideRootScale" null null))
        (set `self.IsBuilding` false)
        (`Widget.RemoveFromParent` (`self.UI_pai`))
        (bind _asbp_human (cast `/Game/HumanDenfense/BluePrint/Aline/Attack/BP_Human` _returnvalue_2)
          (:`then`
            (set `/Game/HumanDenfense/BluePrint/Aline/Attack/BP_Human.Level` _jg_alinebuild_level _asbp_human)
            (set `/Game/HumanDenfense/BluePrint/Aline/Attack/BP_Human.StarLevel` _jg_alinebuild_starlevel _asbp_human))
          (:`CastFailed`
            (bind _asbp_buff (cast `/Game/HumanDenfense/BluePrint/Aline/Buff/BP_Buff` _returnvalue_2)
              (:`then`
                (set `/Game/HumanDenfense/BluePrint/Aline/Buff/BP_Buff.Level` _jg_alinebuild_level _asbp_buff)
                (set `/Game/HumanDenfense/BluePrint/Aline/Buff/BP_Buff.StarLevel` _jg_alinebuild_starlevel _asbp_buff))
              (:`CastFailed`
                (bind _asbp_gold_maker_base (cast `/Game/HumanDenfense/BluePrint/Aline/GoldMaker/BP_GoldMakerBase` _returnvalue_2)
                  (:`then`
                    (set `/Game/HumanDenfense/BluePrint/Aline/GoldMaker/BP_GoldMakerBase.Level` _jg_alinebuild_level _asbp_gold_maker_base)
                    (set `/Game/HumanDenfense/BluePrint/Aline/GoldMaker/BP_GoldMakerBase.StarLevel` _jg_alinebuild_starlevel _asbp_gold_maker_base))
                  (:`CastFailed`
                    (bind _asbp_exp_uper_base (cast `/Game/HumanDenfense/BluePrint/Aline/ExpUper/BP_ExpUperBase` _returnvalue_2))
                    (set `/Game/HumanDenfense/BluePrint/Aline/ExpUper/BP_ExpUperBase.Level` _jg_alinebuild_level _asbp_exp_uper_base)
                    (set `/Game/HumanDenfense/BluePrint/Aline/ExpUper/BP_ExpUperBase.StarLevel` _jg_alinebuild_starlevel _asbp_exp_uper_base))))))))))
  (:`Moved`
    (if (`self.CanMove`)
      (bind _outhit_2 (`KismetSystemLibrary.LineTraceSingleForObjects` :`Start` _worldlocation_2 :`End` (+ (* _worlddirection_2 4000.0) _worldlocation_2) :`ObjectTypes` (`|MakeArray` "ObjectTypeQuery1" :!type "EObjectTypeQuery Enum") :`DrawDebugType` "ForDuration"))
      (`self.K2_SetActorLocation` (`self.DragRef`) (`.Location` (`GameplayStatics.BreakHitResult` _outhit_2)) false false))))

(fn `Fuc_Build`
  (bind (_jg_alinebuild_image _jg_alinebuild_classref _jg_alinebuild_level _jg_alinebuild_starlevel _jg_alinebuild_mesh) (break `/Game/HumanDenfense/BluePrint/JG_PAI` (`self.JG_AlineBuild`)))
  (bind _skeletalmesh (`/Game/HumanDenfense/BluePrint/BP_DragSlot.SkeletalMesh` (`self.DragRef`)))
  (`SkinnedMeshComponent.SetSkinnedAssetAndUpdate` _skeletalmesh _jg_alinebuild_mesh true)
  (`PrimitiveComponent.SetMaterial` _skeletalmesh 0 "/Game/HumanDenfense/material/Build.Build"))

(fn `Fuc_Select`
  (returns (jg :type "/Game/HumanDenfense/BluePrint/JG_PAI Structure") (CanBuild :type Boolean))
  (locals (StarLevel :type Integer :default 0) (Level :type Integer))
  (bind _returnvalue (`KismetMathLibrary.RandomIntegerInRange` 1 100))
  (bind _class (`self.class`))
  (bind _base (`self.Base`))
  (bind _returnvalue_2 (`KismetMathLibrary.RandomIntegerInRange` 0 (- (`KismetArrayLibrary.Array_Length` _class) 1)))
  (if (>= (`/Game/HumanDenfense/BluePrint/Aline/Base/BP_Base.TotalGold` (`self.Base`)) 500)
    (set `/Game/HumanDenfense/BluePrint/Aline/Base/BP_Base.TotalGold` (- (`/Game/HumanDenfense/BluePrint/Aline/Base/BP_Base.TotalGold` _base) 500) _base)
    (if (<= _returnvalue 50)
      (set `local.StarLevel` 1)
      (set `local.Level` 10)
      (elif (<= _returnvalue 80)
        (set `local.StarLevel` 2)
        (set `local.Level` 20)
        (else
          (set `local.StarLevel` 3)
          (set `local.Level` 30))))
    (return (make `/Game/HumanDenfense/BluePrint/JG_PAI` (`|GetArrayItem` (`self.iamge`) _returnvalue_2) (`|GetArrayItem` _class _returnvalue_2) (`local.Level`) (`local.StarLevel`) (`|GetArrayItem` (`self.mesh`) _returnvalue_2)) true)
    (else
      (`KismetSystemLibrary.PrintString` "火柴人不够了  赶快去造呀！！！！！！！！！！！！！！！！！！！！！！！！" true true (struct :`R` 0.040648 :`G` 1.0 :`B` 0.224181 :`A` 1.0))
      (return (struct) false))))

(fn `UserConstructionScript`)