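; BP_B is an enemy Blueprint in HumanDenfense that defines how much damage this enemy type deals to the base.
; Its BaseDamage event subtracts a fixed amount from the HP of the referenced BPBase, with no clamping or death check here.
; BeginPlay, overlap and Tick are unused disabled stubs, and the construction script only calls its parent, so this graph does not show what triggers the damage.
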(event `self.BaseDamage`
  (bind _bp_base (`self.BP_base`))
  (set `/Game/HumanDenfense/BluePrint/Aline/Base/BP_Base.HP` (- (`/Game/HumanDenfense/BluePrint/Aline/Base/BP_Base.HP` _bp_base) 3.0) _bp_base))

(fn `UserConstructionScript`
  (`parent.UserConstructionScript`))