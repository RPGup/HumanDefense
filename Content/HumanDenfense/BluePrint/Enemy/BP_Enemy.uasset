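; Enemy for a human-defense game that marches on BP_Base, scales stats exponentially by wave and awards Exp on death.
; A looping timer box-traces for targets, using skill range when SkillReady, then triggers Attack or Skill montages whose notifies call HitActor or the empty SkillBody hook.
; Armor-reduced, clamped damage updates the health-bar widget, with radial damage accepted only from BP_Human.
; Jitui offsets the enemy for knockback, and Chaofeng redirects it as a taunt.
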(event `BeginSearch`
  (if (`self.CanAttack`) :!label _label
    (bind _returnvalue (`KismetSystemLibrary.K2_SetTimer` self "Fuc_AlineSearch" (`self.SearchDelay`) true))
    (set `self.SearchTimer` _returnvalue)))

(event `self.ReceiveBeginPlay`
  (bind _outactors (`GameplayStatics.GetAllActorsOfClass` "/Game/HumanDenfense/BluePrint/Aline/Base/BP_Base.BP_Base_C"))
  (set `self.HP` (`self.MaxHP`))
  (bind _output (`|GetArrayItem` _outactors))
  (set `self.BP_base` _output)
  (`|AIMoveTo` self (0.0 0.0 0.0) _output 50.0
    (:`then`
      (goto _label))))

(event `WaveUp`
  (params (wave :type Integer))
  (bind _returnvalue (`KismetMathLibrary.MultiplyMultiply_FloatFloat` 1.25 (`KismetMathLibrary.Conv_IntToDouble` wave)))
  (bind _returnvalue_2 (* (`self.MaxHP`) _returnvalue))
  (set `self.MaxHP` _returnvalue_2)
  (set `self.HP` _returnvalue_2)
  (set `self.AttackDamage` (* (`self.AttackDamage`) _returnvalue))
  (set `self.Exp` (`KismetMathLibrary.Round` (* (`self.Exp`) _returnvalue))))

(event `Jitui`
  (params (Impluse :type "Vector Structure"))
  (`self.K2_AddActorWorldOffset` Impluse))

(event `self.ReceiveAnyDamage`
  (params (Damage :type "Float (single-precision)") (DamageType :type "DamageType Object Reference") (InstigatedBy :type "Controller Object Reference") (DamageCauser :type "Actor Object Reference"))
  (bind _hp (`self.HP`))
  (set `self.HP` (- (`self.HP`) (`KismetMathLibrary.FClamp` (- Damage (`self.amor`)) 0.1 10.0)))
  (bind _asui_heath_bar (cast `/Game/HumanDenfense/UI/Pawn/UI_HeathBar` (`WidgetComponent.GetUserWidgetObject` (`self.Health`))))
  (set `/Game/HumanDenfense/UI/Pawn/UI_HeathBar.HP` (/ _hp (`self.MaxHP`)) _asui_heath_bar)
  (if (<= _hp 0.0)
    (`KismetSystemLibrary.PrintString` "Death")
    (`self.EXPUP`)
    (`self.K2_DestroyActor`)))

(event `self.ReceiveRadialDamage`
  (params (DamageReceived :type "Float (single-precision)") (DamageType :type "DamageType Object Reference") (Origin :type "Vector Structure") (HitInfo :type "HitResult Structure (by ref)") (InstigatedBy :type "Controller Object Reference") (DamageCauser :type "Actor Object Reference"))
  (bind _hp (`self.HP`))
  (cast `/Game/HumanDenfense/BluePrint/Aline/Attack/BP_Human` DamageCauser)
  (set `self.HP` (- (`self.HP`) (`KismetMathLibrary.FClamp` (- DamageReceived (`self.amor`)) 0.1 10.0)))
  (bind _asui_heath_bar (cast `/Game/HumanDenfense/UI/Pawn/UI_HeathBar` (`WidgetComponent.GetUserWidgetObject` (`self.Health`))))
  (set `/Game/HumanDenfense/UI/Pawn/UI_HeathBar.HP` (/ _hp (`self.MaxHP`)) _asui_heath_bar)
  (if (<= _hp 0.0)
    (`KismetSystemLibrary.PrintString` "Death")
    (`self.EXPUP`)
    (`self.K2_DestroyActor`)))

(event `Attack`
  (if (not (`self.IsIndebuff`))
    (`MovementComponent.StopMovementImmediately` (`self.CharacterMovement`))
    (`|AIMoveTo` self (0.0 0.0 0.0) (`self.Ref_SearchedAline`) 50.0
      (:`OnSuccess`
        _)
      (:`OnFail`
        _))
    (`|PlayMontage` (`self.Mesh`) "/Game/Mannequin/Animations/Aline_Montage.Aline_Montage" 1.0 0.0 "attack" :!label _label_2
      (:`then`
        (`KismetSystemLibrary.PrintString` "attack" true true (struct :`R` 1.0 :`A` 1.0))
        (`/Engine/EditorBlueprintResources/StandardMacros.IsValid` (`self.Ref_SearchedAline`)
          (:`Is Valid`
            (`KismetSystemLibrary.Delay` (`self.AttackDelay`))
            (goto _label_2))
          (:`Is Not Valid`
            (`KismetSystemLibrary.Delay` (`self.AttackDelay`))
            (bind _returnvalue (`KismetSystemLibrary.K2_SetTimer` self "Fuc_AlineSearch" (`self.SearchDelay`) true))
            (set `self.SearchTimer` _returnvalue)
            (`|AIMoveTo` self (0.0 0.0 0.0) (`self.BP_base`)))))
      (:`OnNotifyBegin`
        (`self.HitActor`)))))

(event `Skill`
  (if (not (`self.IsIndebuff`))
    (`MovementComponent.StopMovementImmediately` (`self.CharacterMovement`))
    (`|AIMoveTo` self (0.0 0.0 0.0) (`self.Ref_SearchedAline`) 50.0
      (:`OnSuccess`
        _)
      (:`OnFail`
        _))
    (`|PlayMontage` (`self.Mesh`) "/Game/Mannequin/Animations/Aline_Montage.Aline_Montage" 1.0 0.0 "attack"
      (:`then`
        (`KismetSystemLibrary.PrintString` "Skill" true true (struct :`R` 1.0 :`A` 1.0))
        (`KismetSystemLibrary.Delay` (`self.AttackDelay`))
        (bind _returnvalue (`KismetSystemLibrary.K2_SetTimer` self "Fuc_AlineSearch" (`self.SearchDelay`) true))
        (set `self.SearchTimer` _returnvalue)
        (bind _returnvalue_2 (`KismetSystemLibrary.K2_SetTimerDelegate` (delegate `SkillReset`) (`self.SkillDelay`) true))
        (set `self.SkillResetTimer` _returnvalue_2)
        (`|AIMoveTo` self (0.0 0.0 0.0) (`self.BP_base`)))
      (:`OnNotifyBegin`
        (`self.SkillBody`)))))

(event `SkillReset`
  (set `self.SkillReady` true))

(event `HitActor`
  (`GameplayStatics.ApplyDamage` (`self.Ref_SearchedAline`) (`self.AttackDamage`)))

(event `SkillBody`)

(event `Chaofeng`
  (params (ChaofengMan :type "Actor Object Reference") (Time :type "Float (double-precision)"))
  (set `self.IsIndebuff` false)
  (`MovementComponent.StopMovementImmediately` (`self.CharacterMovement`))
  (`|AIMoveTo` self (0.0 0.0 0.0) ChaofengMan 50.0
    (:`then`
      (`KismetSystemLibrary.Delay` Time)
      (set `self.IsIndebuff` true))
    (:`OnSuccess`
      (`self.Attack`))))

(event `EXPUP`
  (bind _exp (`self.Exp`))
  (bind _outactors (`GameplayStatics.GetAllActorsOfClass` "/Game/HumanDenfense/BluePrint/Aline/Attack/BP_Human.BP_Human_C"))
  (for _array_element _outactors
    (`/Game/HumanDenfense/BluePrint/Aline/Attack/BP_Human.CaculateExp` _array_element _exp))
  (bind _outactors_2 (`GameplayStatics.GetAllActorsOfClass` "/Game/HumanDenfense/BluePrint/Aline/GoldMaker/BP_GoldMakerBase.BP_GoldMakerBase_C"))
  (for _array_element_2 _outactors_2
    (`/Game/HumanDenfense/BluePrint/Aline/GoldMaker/BP_GoldMakerBase.CaculateExp` _array_element_2 _exp))
  (bind _outactors_3 (`GameplayStatics.GetAllActorsOfClass` "/Game/HumanDenfense/BluePrint/Aline/Buff/BP_Buff.BP_Buff_C"))
  (for _array_element_3 _outactors_3
    (`/Game/HumanDenfense/BluePrint/Aline/Buff/BP_Buff.CaculateExp` _array_element_3 0))
  (bind _outactors_4 (`GameplayStatics.GetAllActorsOfClass` "/Game/HumanDenfense/BluePrint/Aline/ExpUper/BP_ExpUperBase.BP_ExpUperBase_C"))
  (for _array_element_4 _outactors_4
    (`/Game/HumanDenfense/BluePrint/Aline/ExpUper/BP_ExpUperBase.CaculateEXP` _array_element_4 _exp)))

(fn `Fuc_AlineSearch`
  (bind _returnvalue (`self.K2_GetActorLocation`))
  (bind _attackrange (`self.AttackRange`))
  (if (`self.SkillReady`)
    (`self.Fuc_SkillSearch`)
    (else
      (bind (_outhit _returnvalue_2) (`KismetSystemLibrary.BoxTraceSingleForObjects` :`Start` _returnvalue :`End` (+ (* (`KismetMathLibrary.GetForwardVector` (`self.K2_GetActorRotation`)) _attackrange) _returnvalue) :`HalfSize` (`KismetMathLibrary.MakeVector` _attackrange _attackrange 50.0) :`Orientation` (struct :`Yaw` 45.0) :`ObjectTypes` (`|MakeArray` "ObjectTypeQuery7" :!type "EObjectTypeQuery Enum") :`DrawDebugType` "ForDuration"))
      (if _returnvalue_2
        (`KismetSystemLibrary.K2_ClearAndInvalidateTimerHandle` (`self.SearchTimer`))
        (set `self.Ref_SearchedAline` (`.HitActor` (`GameplayStatics.BreakHitResult` _outhit)))
        (`self.Attack`)
        (return)))))

(fn `Fuc_SkillSearch`
  (bind _returnvalue (`self.K2_GetActorLocation`))
  (bind _skillrange (`self.SkillRange`))
  (bind (_outhit _returnvalue_2) (`KismetSystemLibrary.BoxTraceSingleForObjects` :`Start` _returnvalue :`End` (+ (* (`KismetMathLibrary.GetForwardVector` (`self.K2_GetActorRotation`)) _skillrange) _returnvalue) :`HalfSize` (`KismetMathLibrary.MakeVector` _skillrange _skillrange 50.0) :`Orientation` (struct :`Yaw` 45.0) :`ObjectTypes` (`|MakeArray` "ObjectTypeQuery7" :!type "EObjectTypeQuery Enum") :`DrawDebugType` "ForDuration"))
  (if _returnvalue_2
    (`KismetSystemLibrary.K2_ClearAndInvalidateTimerHandle` (`self.SearchTimer`))
    (`KismetSystemLibrary.K2_ClearAndInvalidateTimerHandle` (`self.SkillResetTimer`))
    (set `self.Ref_SearchedAline` (`.HitActor` (`GameplayStatics.BreakHitResult` _outhit)))
    (`self.Skill`)
    (set `self.SkillReady` false)
    (return)))

(fn `UserConstructionScript`)