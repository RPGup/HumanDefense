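; BP_KL is a GoldMaker unit Blueprint whose gold amount (GoldNum) grows with its star level.
; Its Star++ event raises StarLevel up to a cap of five, writes the new star to the UI_Health widget in HPANDEXP, then sets GoldNum from a per-level table.
; A failed widget cast blocks the upgrade entirely.
; BeginPlay, overlap and Tick are disabled stubs, so this graph only handles upgrades.
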(event `self.Star++`
  (bind _returnvalue (+ (`self.StarLevel`) 1))
  (if (not (== (`self.StarLevel`) 5))
    (bind _asui_health (cast `/Game/HumanDenfense/UI/aLINE/UI_Health` (`WidgetComponent.GetUserWidgetObject` (`self.HPANDEXP`))))
    (set `/Game/HumanDenfense/UI/aLINE/UI_Health.Star` _returnvalue _asui_health)
    (bind _output_get (set `self.StarLevel` _returnvalue))
    (switch `int` _output_get
      (:`1`
        (set `self.GoldNum` 100))
      (:`2`
        (set `self.GoldNum` 200))
      (:`3`
        (set `self.GoldNum` 400))
      (:`4`
        (set `self.GoldNum` 700))
      (:`5`
        (set `self.GoldNum` 1500)))))

(fn `UserConstructionScript`
  (`parent.UserConstructionScript`))