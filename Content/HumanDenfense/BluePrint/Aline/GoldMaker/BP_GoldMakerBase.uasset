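; BP_GoldMakerBase is a gold-producing allied unit that earns gold for the base while it has a deposit.
; On BeginPlay it sphere-traces for BP_Gold, claims the nearest within range, then runs a looping timer that credits BP_Base and plays an attack montage.
; Experience raises level and HP up to a StarLevel-based cap, though Star++ is an empty stub.
; Only BP_Enemy damage lowers HP, which updates the widget and destroys the actor at zero.
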(event `self.ReceiveBeginPlay`
  (bind _returnvalue (`self.K2_GetActorLocation`))
  (bind _outhits (`KismetSystemLibrary.SphereTraceMultiForObjects` :`Start` _returnvalue :`End` _returnvalue :`Radius` (`self.SearchRadius`) :`ObjectTypes` (`|MakeArray` "ObjectTypeQuery11" :!type "EObjectTypeQuery Enum") :`DrawDebugType` "ForDuration"))
  (`KismetArrayLibrary.Array_Clear` (`self.Ref_SearchedGold`))
  (for _array_element _outhits
    (bind _asbp_gold (cast `/Game/HumanDenfense/BluePrint/Aline/Base/BP_Gold` (`.HitActor` (`GameplayStatics.BreakHitResult` _array_element))))
    (`KismetArrayLibrary.Array_Add` (`self.Ref_SearchedGold`) _asbp_gold))
  (bind _isfind (`self.FindGold`))
  (if _isfind
    (bind _asbp_gold_2 (cast `/Game/HumanDenfense/BluePrint/Aline/Base/BP_Gold` (`self.Ref_Gold`)))
    (set `/Game/HumanDenfense/BluePrint/Aline/Base/BP_Gold.Ref_GoldMaker` self _asbp_gold_2)
    (bind _outactors (`GameplayStatics.GetAllActorsOfClass` "/Game/HumanDenfense/BluePrint/Aline/Base/BP_Base.BP_Base_C"))
    (set `self.Ref_Base` (`|GetArrayItem` _outactors))
    (`KismetSystemLibrary.K2_SetTimerDelegate` (delegate `MakeGold`) (`self.GoldMakeDelay`) true)))

(event `MakeGold`
  (`/Game/HumanDenfense/BluePrint/Aline/Base/BP_Base.CaculateGold` (`self.Ref_Base`) (`self.GoldNum`))
  (`|PlayMontage` (`self.Mesh`) "/Game/Mannequin/Animations/Aline_Montage.Aline_Montage" 1.0 0.0 "attack"))

(event `LevelUp`
  (bind _asui_health (cast `/Game/HumanDenfense/UI/Pawn/UI_Health` (`WidgetComponent.GetUserWidgetObject` (`self.HPANDEXP`))))
  (set `/Game/HumanDenfense/UI/Pawn/UI_Health.Level` (`self.Level`) _asui_health)
  (set `self.HP` (+ (`self.HP`) (`self.HPUP`)))
  (set `self.MaxHp` (+ (`self.HPUP`) (`self.MaxHp`))))

(event `self.ReceiveAnyDamage`
  (params (Damage :type "Float (single-precision)") (DamageType :type "DamageType Object Reference") (InstigatedBy :type "Controller Object Reference") (DamageCauser :type "Actor Object Reference"))
  (cast `/Game/HumanDenfense/BluePrint/Enemy/BP_Enemy` DamageCauser)
  (`self.CaculateHP` Damage))

(event `Star++`)

(fn `CaculateExp`
  (params (Exp :type Integer))
  (bind _exp (`self.Exp`))
  (if (== (* (`self.StarLevel`) 10) (`self.Level`))
    (`KismetSystemLibrary.PrintString` "CanNotGetExp")
    (else
      (set `self.Exp` (+ Exp (`self.Exp`)))
      (if (>= _exp (`self.LevelExp`)) :!label _label
        (set `self.Exp` (- _exp (`self.LevelExp`)))
        (set `self.Level` (+ (`self.Level`) 1))
        (`self.LevelUp`)
        (if (== (* (`self.StarLevel`) 10) (`self.Level`))
          (set `self.Exp` 0)
          (else
            (goto _label))))
      (bind _asui_health (cast `/Game/HumanDenfense/UI/Pawn/UI_Health` (`WidgetComponent.GetUserWidgetObject` (`self.HPANDEXP`))))
      (`ProgressBar.SetPercent` (`/Game/HumanDenfense/UI/Pawn/UI_Health.ExpBar` _asui_health) (/ (`KismetMathLibrary.Conv_IntToDouble` (`self.Exp`)) (`KismetMathLibrary.Conv_IntToDouble` (`self.LevelExp`))))
      (return))))

(fn `CaculateHP`
  (params (A :type "Float (double-precision)"))
  (bind _maxhp (`self.MaxHp`))
  (bind _output_get (set `self.HP` (- (`self.HP`) A)))
  (bind _asui_health (cast `/Game/HumanDenfense/UI/Pawn/UI_Health` (`WidgetComponent.GetUserWidgetObject` (`self.HPANDEXP`))))
  (`ProgressBar.SetPercent` (`/Game/HumanDenfense/UI/Pawn/UI_Health.HealthBar` _asui_health) (/ _output_get (`self.MaxHp`)))
  (if (<= _output_get 0.0)
    (`self.K2_DestroyActor`)
    (`KismetSystemLibrary.PrintString` "death")
    (elif (>= (`self.HP`) _maxhp)
      (set `self.HP` _maxhp)))
  (return))

(fn `FindGold`
  (returns (isFind :type Boolean))
  (locals (Destance :type "Float (double-precision)" :default 9999.0))
  (for _array_element (`self.Ref_SearchedGold`)
    (if (`KismetSystemLibrary.IsValid` _array_element)
      (bind _returnvalue (`KismetMathLibrary.VSize` (- (`self.K2_GetActorLocation` _array_element) (`self.K2_GetActorLocation`))))
      (if (<= _returnvalue (`local.Destance`))
        (set `local.Destance` _returnvalue)
        (set `self.Ref_Gold` _array_element))))
  (return (`KismetSystemLibrary.IsValid` (`self.Ref_Gold`))))

(fn `UserConstructionScript`)