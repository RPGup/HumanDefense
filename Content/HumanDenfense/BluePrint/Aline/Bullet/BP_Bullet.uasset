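; BP_Bullet is a projectile Blueprint that damages enemies in the HumanDenfense game.
; On overlap it casts the other actor to BP_Enemy and only reacts if that enemy is its assigned RefAttacking target, ignoring all others.
; On a valid hit it applies Damage to the enemy, spawns an explosion emitter at its location and destroys itself.
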(event `self.Overlap`
  (params (OverlapActor :type "Actor Object Reference"))
  (bind _asbp_enemy (cast `/Game/HumanDenfense/Enemy/BP_Enemy` OverlapActor))
  (if (== _asbp_enemy (`self.Ref_Attacking`))
    (`GameplayStatics.ApplyDamage` _asbp_enemy (`self.Damage`) null self)
    (`GameplayStatics.SpawnEmitterAtLocation` "/Game/StarterContent/Particles/P_Explosion.P_Explosion" (`self.K2_GetActorLocation`))
    (`self.K2_DestroyActor`)))

(fn `UserConstructionScript`
  (`parent.UserConstructionScript`))