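; BP_Skill03 is a bullet-type skill actor that triggers a follow-up YFY skill effect when it reaches its target enemy.
; On Overlap, it casts the actor to BP_Enemy and acts only if it matches RefAttacking.
; It then spawns BP_YFYskill03 at that enemy's location, passing on explosion radius, damage and damage delay.
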(event `self.Overlap`
  (params (OverlapActor :type "Actor Object Reference"))
  (bind _asbp_enemy (cast `/Game/HumanDenfense/Enemy/BP_Enemy` OverlapActor))
  (if (== _asbp_enemy (`self.Ref_Attacking`))
    (bind _returnvalue (`self.K2_GetActorLocation` _asbp_enemy))
    (`|SpawnActorFromClass` "/Game/HumanDenfense/BluePrint/Aline/Bullet/YFY/BP_YFYskill03.BP_YFYskill03_C" (`KismetMathLibrary.MakeTransform` _returnvalue) "Undefined" "OverrideRootScale" null _returnvalue (`self.ExpRadius`) (`self.Damage`) (`self.DamageDelay`) null)))

(fn `UserConstructionScript`
  (`parent.UserConstructionScript`))