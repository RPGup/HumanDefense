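; BP_YFYskill02 is an explosive skill projectile for the YFY Aline character that damages an area around its target enemy.
; Its Overlap event ignores everything except the BP_Enemy stored in RefAttacking.
; On that hit it applies full radial damage within ExposionRadius, credited to RefAline, spawns an explosion particle and destroys itself.
; An unconnected sphere-trace damage branch remains in the graph and never runs.
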(event `self.ReceiveBeginPlay`
  (`parent.ReceiveBeginPlay`))

(event `self.Overlap`
  (params (OverlapActor :type "Actor Object Reference"))
  (bind _particlelocation (`self.ParticleLocation`))
  (bind _asbp_enemy (cast `/Game/HumanDenfense/Enemy/BP_Enemy` OverlapActor))
  (if (== _asbp_enemy (`self.Ref_Attacking`))
    (set `self.ParticleLocation` (`self.K2_GetActorLocation` _asbp_enemy))
    (`GameplayStatics.ApplyRadialDamage` :`BaseDamage` (`self.Damage`) :`Origin` _particlelocation :`DamageRadius` (`self.ExposionRadius`) :`DamageCauser` (`self.Ref_Aline`) :`InstigatedByController` null :`bDoFullDamage` true :`DamagePreventionChannel` "ECC_GameTraceChannel1")
    (`GameplayStatics.SpawnEmitterAtLocation` "/Game/StarterContent/Particles/P_Explosion.P_Explosion" _particlelocation)
    (`self.K2_DestroyActor`)))

(fn `UserConstructionScript`
  (`parent.UserConstructionScript`))