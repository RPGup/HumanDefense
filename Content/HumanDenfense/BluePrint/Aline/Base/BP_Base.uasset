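; BP_Base is a base Blueprint in the HumanDenfense game that keeps a running gold total.
; CaculateGold adds the given amount to TotalGold, prints it on screen, then casts player controller 0 to BP_PlayerContol and writes the total to the Gold value of its Main object.
; Its event graph and construction script contain no logic.
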(fn `CaculateGold`
  (params (gold :type Integer))
  (bind _output_get (set `self.TotalGold` (+ gold (`self.TotalGold`))))
  (`KismetSystemLibrary.PrintString` (`KismetStringLibrary.Conv_IntToString` _output_get))
  (bind _asbp_player_contol (cast `/Game/HumanDenfense/BluePrint/BP_PlayerContol` (`GameplayStatics.GetPlayerController` 0)))
  (set `/Game/HumanDenfense/UI/Main.Gold` (`self.TotalGold`) (`/Game/HumanDenfense/BluePrint/BP_PlayerContol.Main` _asbp_player_contol))
  (return))

(fn `UserConstructionScript`)