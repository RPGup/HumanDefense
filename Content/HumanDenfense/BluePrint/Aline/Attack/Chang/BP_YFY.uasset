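; BP_YFY is an attacking unit that fires at RefFirstEnemy from Arrow1, with attacks that grow with SkillLevel.
; Attackto picks the highest ready attack: Skill03 projectile, boosted Skill01 bullet, then a basic shot, which becomes an explosive Skill02 projectile from level two.
; Skill01–03 events each set their level once.
; Looping timers, restarted on use, re-arm the Skill01 and Skill03 cooldown flags.
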(event `self.AttackTo`
  (switch `int` (`self.SkillLevel`)
    (:`0`
      (`|SpawnActorFromClass` "/Game/HumanDenfense/BluePrint/Aline/Bullet/BP_Bullet.BP_Bullet_C" (`SceneComponent.K2_GetComponentToWorld` (`self.Arrow1`)) "Undefined" "OverrideRootScale" null (`self.NomalDamage`) (`self.Ref_FirstEnemy`) null :!label _label))
    (:`1`
      (if (`self.Skill01Ready`)
        (`KismetSystemLibrary.K2_ClearAndInvalidateTimerHandle` (`self.Skill01Timer`) :!label _label_2)
        (bind _returnvalue (`KismetSystemLibrary.K2_SetTimerDelegate` (delegate `Skill01Reset`) (`self.Skill01Delay`) true))
        (set `self.Skill01Timer` _returnvalue)
        (`|SpawnActorFromClass` "/Game/HumanDenfense/BluePrint/Aline/Bullet/BP_Bullet.BP_Bullet_C" (`SceneComponent.K2_GetComponentToWorld` (`self.Arrow1`)) "Undefined" "OverrideRootScale" null (* (`self.NomalDamage`) 2.5) (`self.Ref_FirstEnemy`) null)
        (`KismetSystemLibrary.PrintString` "Skill01")
        (set `self.Skill01Ready` false)
        (else
          (goto _label))))
    (:`2`
      (if (`self.Skill01Ready`)
        (goto _label_2)
        (else
          (`|SpawnActorFromClass` "/Game/HumanDenfense/BluePrint/Aline/Bullet/YFY/BP_YFYskill02.BP_YFYskill02_C" (`SceneComponent.K2_GetComponentToWorld` (`self.Arrow1`)) "Undefined" "OverrideRootScale" null (`self.Skill02ExpRadius`) null (`self.NomalDamage`) (`self.Ref_FirstEnemy`) null :!label _label_3))))
    (:`3`
      (if (`self.Skill03Ready`)
        (`KismetSystemLibrary.K2_ClearAndInvalidateTimerHandle` (`self.Skill03Timer`))
        (bind _returnvalue_2 (`KismetSystemLibrary.K2_SetTimerDelegate` (delegate `Skill03Reset`) (`self.Skill03Delay`) true))
        (set `self.Skill03Timer` _returnvalue_2)
        (`|SpawnActorFromClass` "/Game/HumanDenfense/BluePrint/Aline/Bullet/YFY/BP_Skill03.BP_Skill03_C" (`SceneComponent.K2_GetComponentToWorld` (`self.Arrow1`)) "Undefined" "OverrideRootScale" null (`self.ExpRadius`) (`self.DamageDelay`) (* (`self.NomalDamage`) 3.0) (`self.Ref_FirstEnemy`) null)
        (set `self.Skill03Ready` false)
        (`KismetSystemLibrary.PrintString` "Skill03")
        (elif (`self.Skill01Ready`)
          (goto _label_2)
          (else
            (goto _label_3)))))))

(event `self.Skill01`
  (`/Engine/EditorBlueprintResources/StandardMacros.DoOnce` false
    (:`Completed`
      (set `self.SkillLevel` 1)
      (bind _returnvalue (`KismetSystemLibrary.K2_SetTimerDelegate` (delegate `Skill01Reset`) (`self.Skill01Delay`) true))
      (set `self.Skill01Timer` _returnvalue))))

(event `Skill01Reset`
  (set `self.Skill01Ready` true))

(event `self.Skill02`
  (`/Engine/EditorBlueprintResources/StandardMacros.DoOnce` false
    (:`Completed`
      (set `self.SkillLevel` 2))))

(event `self.Skill03`
  (`/Engine/EditorBlueprintResources/StandardMacros.DoOnce` false
    (:`Completed`
      (set `self.SkillLevel` 3)
      (bind _returnvalue (`KismetSystemLibrary.K2_SetTimerDelegate` (delegate `Skill03Reset`) (`self.Skill03Delay`) true))
      (set `self.Skill03Timer` _returnvalue))))

(event `Skill03Reset`
  (set `self.Skill03Ready` true))

(fn `UserConstructionScript`
  (`parent.UserConstructionScript`))