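; BP_Human is a defender character that automatically fights enemies near the base, with health, armor, experience and star-capped levels shown in UI_Health.
; A delayed Search loop sphere-traces for enemies and favors those closest to BP_Base.
; Mobile units chase within range of their spawn point and return, while stationary ones play attack montages.
; XuanYun stuns temporarily, and AttackTo and the level 10/30/50 skills are empty hooks.
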(event `self.ReceiveBeginPlay`
  (bind _outactors (`GameplayStatics.GetAllActorsOfClass` "/Game/HumanDenfense/BluePrint/Aline/Base/BP_Base.BP_Base_C"))
  (set `self.Ref_Base` (`|GetArrayItem` _outactors))
  (`self.Search`)
  (set `self.wordlocation` (`self.K2_GetActorLocation`))
  (if (== (`self.Level`) 10)
    (`self.Skill01`)
    (elif (== (`self.Level`) 30)
      (`self.Skill02`)
      (elif (== (`self.Level`) 50)
        (`self.Skill03`)))))

(event `Search`
  (bind _returnvalue (`self.K2_GetActorLocation`))
  (bind _wordlocation (`self.wordlocation`))
  (bind _ref_searchedenemy (`self.Ref_SearchedEnemy`))
  (`KismetSystemLibrary.Delay` (`self.AttackDelay`))
  (if (`self.IsInDebuff`)
    _
    (elif (`self.CanMove`)
      (if (and (not (`self.isbacking?`)) (`self.IsNotMoving`))
        (bind (_outhits _returnvalue_2) (`KismetSystemLibrary.SphereTraceMultiForObjects` :`Start` _wordlocation :`End` _wordlocation :`Radius` (`self.MoveRange`) :`ObjectTypes` (`|MakeArray` "ObjectTypeQuery8" :!type "EObjectTypeQuery Enum") :`DrawDebugType` "ForDuration"))
        (if _returnvalue_2
          (`KismetArrayLibrary.Array_Clear` (`self.Ref_SearchedEnemy`))
          (for _array_element _outhits
            (`KismetArrayLibrary.Array_Add` _ref_searchedenemy (`.HitActor` (`GameplayStatics.BreakHitResult` _array_element)))
            (`KismetSystemLibrary.PrintString` (`KismetStringLibrary.Conv_IntToString` (`KismetArrayLibrary.Array_Length` _ref_searchedenemy))))
          (if (> (`KismetArrayLibrary.Array_Length` (`self.Ref_SearchedEnemy`)) 0)
            (bind _issearched (`self.FindFirstEnemy`))
            (if _issearched
              (if (> (`KismetMathLibrary.VSize` (- (`self.K2_GetActorLocation`) (`self.wordlocation`))) (`self.MoveRange`))
                (`self.Back`)
                (else
                  (`self.MoveTo`)
                  (`KismetSystemLibrary.PrintString` "Move")))
              (else
                (`self.Search` :!label _label)))
            (else
              (goto _label)))
          (else
            (`self.Back`)))
        (else
          (`KismetSystemLibrary.PrintString` "Hello")))
      (else
        (bind (_outhits_2 _returnvalue_3) (`KismetSystemLibrary.SphereTraceMultiForObjects` :`Start` _returnvalue :`End` _returnvalue :`Radius` (`self.AttackRange`) :`ObjectTypes` (`|MakeArray` "ObjectTypeQuery8" :!type "EObjectTypeQuery Enum") :`DrawDebugType` "ForDuration"))
        (if _returnvalue_3
          (`KismetArrayLibrary.Array_Clear` (`self.Ref_SearchedEnemy`))
          (for _array_element_2 _outhits_2
            (`KismetArrayLibrary.Array_Add` (`self.Ref_SearchedEnemy`) (`.HitActor` (`GameplayStatics.BreakHitResult` _array_element_2))))
          (if (> (`KismetArrayLibrary.Array_Length` (`self.Ref_SearchedEnemy`)) 0)
            (bind _issearched_2 (`self.FindFirstEnemy`))
            (if _issearched_2
              (`self.AttackNormal`)
              (else
                (`self.Search` :!label _label_2)))
            (else
              (goto _label_2)))
          (else
            (`self.Search`)))))))

(event `AttackNormal`
  (bind _ref_firstenemy (`self.Ref_FirstEnemy`))
  (bind (_returnvalue_roll _returnvalue_pitch _returnvalue_yaw) (`KismetMathLibrary.BreakRotator` (`KismetMathLibrary.FindLookAtRotation` (`self.K2_GetActorLocation`) (`self.K2_GetActorLocation` (`self.Ref_FirstEnemy`)))))
  (if (not (`self.IsInDebuff`))
    (`self.K2_SetActorRotation` (`KismetMathLibrary.MakeRotator` 0.0 0.0 _returnvalue_yaw))
    (`|PlayMontage` (`self.Mesh`) (`self.Ref_Montage`) 1.0 0.0 (`self.StartSection`)
      (:`then`
        (set `self.isAttacking` true))
      (:`OnCompleted`
        (`KismetSystemLibrary.Delay` (`self.AttackDelay`))
        (if (`KismetSystemLibrary.IsValid` _ref_firstenemy)
          (if (> (`KismetMathLibrary.VSize` (- (`self.K2_GetActorLocation` _ref_firstenemy) (`self.K2_GetActorLocation` self))) (`self.AttackRange`))
            (`self.Search` :!label _label_3)
            (set `self.isAttacking` false)
            (else
              (`self.AttackNormal`)))
          (else
            (goto _label_3))))
      (:`OnNotifyBegin`
        (`self.AttackTo`)))))

(event `MoveTo`
  (if (not (`self.IsInDebuff`))
    (set `self.IsNotMoving` false)
    (`|AIMoveTo` self (0.0 0.0 0.0) (`self.Ref_FirstEnemy`) (`self.AttackRange`)
      (:`OnSuccess`
        _)
      (:`OnFail`
        _))
    (set `self.IsNotMoving` true)
    (`self.AttackTo`)
    (`self.Search`)))

(event `Back`
  (if (`self.IsInDebuff`)
    _
    (elif (== (`self.K2_GetActorLocation`) (`self.wordlocation`) :`ErrorTolerance` 0.01)
      (`self.Search` :!label _label_4)
      (else
        (set `CharacterMovementComponent.MaxWalkSpeed` 1500.0 (`self.CharacterMovement`))
        (`|AIMoveTo` self (`self.wordlocation`) null 0.0
          (:`then`
            (set `self.isbacking?` true))
          (:`OnSuccess`
            (set `CharacterMovementComponent.MaxWalkSpeed` (`self.MaxWalkSP`) (`self.CharacterMovement`) :!label _label_5)
            (set `self.isbacking?` false)
            (goto _label_4))
          (:`OnFail`
            (goto _label_5)))))))

(event `LevelUp`
  (bind _asui_health (cast `/Game/HumanDenfense/UI/aLINE/UI_Health` (`WidgetComponent.GetUserWidgetObject` (`self.HPandEXP`))))
  (set `/Game/HumanDenfense/UI/aLINE/UI_Health.Level` (`self.Level`) _asui_health)
  (set `self.NomalDamage` (+ (`self.NomalDamage`) (`self.DamageUP`)))
  (set `self.MaxHp` (+ (`self.HPUP`) (`self.MaxHp`)))
  (set `self.HP` (+ (`self.HPUP`) (`self.HP`)))
  (if (== (`self.Level`) 10)
    (`self.Skill01`)
    (elif (== (`self.Level`) 30)
      (`self.Skill02`)
      (elif (== (`self.Level`) 50)
        (`self.Skill03`)))))

(event `self.ReceiveAnyDamage`
  (params (Damage :type "Float (single-precision)") (DamageType :type "DamageType Object Reference") (InstigatedBy :type "Controller Object Reference") (DamageCauser :type "Actor Object Reference"))
  (cast `/Game/HumanDenfense/BluePrint/Aline/Attack/BP_Human` DamageCauser
    (:`CastFailed`
      (`self.CaculateHP` Damage))))

(event `AttackTo`)

(event `Skill01`)

(event `Skill02`)

(event `Skill03`)

(event `Star+`
  (bind _returnvalue (+ (`self.StarLevel`) 1))
  (if (not (== (`self.StarLevel`) 5))
    (bind _asui_health (cast `/Game/HumanDenfense/UI/aLINE/UI_Health` (`WidgetComponent.GetUserWidgetObject` (`self.HPandEXP`))))
    (set `/Game/HumanDenfense/UI/aLINE/UI_Health.Star` _returnvalue _asui_health)
    (set `self.StarLevel` _returnvalue)))

(event `XuanYun`
  (params (Damage :type "Float (double-precision)") (YunXuanTime :type "Float (double-precision)"))
  (set `self.IsInDebuff` true)
  (`KismetSystemLibrary.PrintString` "xuanyun" true true (struct :`R` 1.0 :`G` 0.92521 :`A` 1.0))
  (`self.StopAnimMontage` "/Game/Mannequin/Animations/Aline_Montage.Aline_Montage")
  (`MovementComponent.StopMovementImmediately` (`self.CharacterMovement`))
  (`self.CaculateHP` Damage)
  (`KismetSystemLibrary.Delay` YunXuanTime)
  (set `self.IsInDebuff` false)
  (`KismetSystemLibrary.Delay` 0.1)
  (`self.Search`))

(fn `CaculateExp`
  (params (Exp :type Integer))
  (bind _exp (`self.Exp`))
  (if (== (* (`self.StarLevel`) 10) (`self.Level`))
    (`KismetSystemLibrary.PrintString` "CanNotGetExp")
    (else
      (set `self.Exp` (+ Exp (`self.Exp`)))
      (if (>= _exp (`self.LevelExp`)) :!label _label
        (set `self.Exp` (- _exp (`self.LevelExp`)))
        (set `self.Level` (+ (`self.Level`) 1))
        (`self.LevelUp`)
        (if (== (* (`self.StarLevel`) 10) (`self.Level`))
          (set `self.Exp` 0)
          (else
            (goto _label))))
      (bind _asui_health (cast `/Game/HumanDenfense/UI/aLINE/UI_Health` (`WidgetComponent.GetUserWidgetObject` (`self.HPandEXP`))))
      (`ProgressBar.SetPercent` (`/Game/HumanDenfense/UI/aLINE/UI_Health.ExpBar` _asui_health) (/ (`KismetMathLibrary.Conv_IntToDouble` (`self.Exp`)) (`KismetMathLibrary.Conv_IntToDouble` (`self.LevelExp`))))
      (return))))

(fn `CaculateHP`
  (params (A :type "Float (double-precision)"))
  (bind _maxhp (`self.MaxHp`))
  (if (<= A 0.0)
    (set `self.HP` (- (`self.HP`) A))
    (else
      (bind _output_get (set `self.HP` (- (`self.HP`) (`KismetMathLibrary.FClamp` (- A (`self.amor`)) 0.1 5.0))))))
  (bind _asui_health (cast `/Game/HumanDenfense/UI/aLINE/UI_Health` (`WidgetComponent.GetUserWidgetObject` (`self.HPandEXP`))))
  (`ProgressBar.SetPercent` (`/Game/HumanDenfense/UI/aLINE/UI_Health.HealthBar` _asui_health) (/ _output_get (`self.MaxHp`)))
  (if (<= _output_get 0.0)
    (`self.K2_DestroyActor`)
    (`KismetSystemLibrary.PrintString` "death")
    (elif (>= _output_get _maxhp)
      (set `self.HP` _maxhp)))
  (return))

(fn `FindFirstEnemy`
  (returns (IsSearched :type Boolean))
  (locals (Destance :type "Float (double-precision)" :default 9999.0))
  (for _array_element (`self.Ref_SearchedEnemy`)
    (if (`KismetSystemLibrary.IsValid` _array_element)
      (bind _returnvalue (`KismetMathLibrary.VSize` (- (`self.K2_GetActorLocation` _array_element) (`self.K2_GetActorLocation` (`self.Ref_Base`)))))
      (if (<= _returnvalue (`local.Destance`))
        (set `local.Destance` _returnvalue)
        (set `self.Ref_FirstEnemy` _array_element))))
  (return (`KismetSystemLibrary.IsValid` (`self.Ref_FirstEnemy`))))

(fn `UserConstructionScript`
  (set `CharacterMovementComponent.MaxWalkSpeed` (`self.MaxWalkSP`) (`self.CharacterMovement`)))