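; BP_longMan is an attacker Blueprint that fires a projectile at an enemy.
; Its Attackto event spawns a BP_NomalBullet at the Arrow1 component's world transform, passing NomalDamage as damage and RefFirstEnemy as the target.
; The BeginPlay, overlap and Tick events are disabled stubs, and the construction script only calls its parent, so this graph adds only the shot.
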(event `self.AttackTo`
  (`|SpawnActorFromClass` "/Game/HumanDenfense/BluePrint/Aline/Bullet/BP_NomalBullet.BP_NomalBullet_C" (`SceneComponent.K2_GetComponentToWorld` (`self.Arrow1`)) "Undefined" "OverrideRootScale" null (`self.NomalDamage`) (`self.Ref_FirstEnemy`) null))

(fn `UserConstructionScript`
  (`parent.UserConstructionScript`))