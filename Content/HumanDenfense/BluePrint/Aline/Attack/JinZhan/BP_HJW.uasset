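; BP_HJW is a melee defender unit with three one-time skill unlocks: armor, area taunt and area knockback.
; Each unlock sets SkillLevel, which Attackto uses to pick the strongest ready skill, falling back to a montage attack that damages RefFirstEnemy on notify.
; Taunt and knockback sphere-trace for BP_Enemy to call Chaofeng or Jitui, with looping timers restoring readiness.
; The knockback path's ApplyDamage follows Jitui, and debug traces remain enabled.
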(event `self.ReceiveBeginPlay`
  (`parent.ReceiveBeginPlay`))

(event `self.Skill01`
  (`/Engine/EditorBlueprintResources/StandardMacros.DoOnce` false
    (:`Completed`
      (set `self.Amor` 1.0)
      (set `self.SkillLevel` 1)
      (`KismetSystemLibrary.PrintString` "Amor1"))))

(event `self.AttackTo`
  (bind _wordlocation (`self.wordlocation`))
  (bind _wordlocation_2 (`self.wordlocation`))
  (switch `int` (`self.SkillLevel`)
    (:`0`
      (`|PlayMontage` (`self.Mesh`) (`self.Ref_Montage`) 1.0 0.0 (`self.StartSection`) :!label _label
        (:`then`
          (set `self.isAttacking` true))
        (:`OnCompleted`
          (set `self.isAttacking` false))
        (:`OnNotifyBegin`
          (`GameplayStatics.ApplyDamage` (`self.Ref_FirstEnemy`) (`self.NomalDamage`) null self))))
    (:`1`
      (goto _label))
    (:`2`
      (if (`self.Skill02Ready`)
        (`KismetSystemLibrary.K2_ClearAndInvalidateTimerHandle` (`self.Skill02Timer`) :!label _label_2)
        (bind _returnvalue (`KismetSystemLibrary.K2_SetTimerDelegate` (delegate `Skill02Reset`) (`self.Skill02Delay`) true))
        (set `self.Skill02Timer` _returnvalue)
        (bind (_outhits _returnvalue_2) (`KismetSystemLibrary.SphereTraceMultiForObjects` :`Start` _wordlocation :`End` _wordlocation :`Radius` (`self.Skill02Range`) :`ObjectTypes` (`|MakeArray` "ObjectTypeQuery8" :!type "EObjectTypeQuery Enum") :`DrawDebugType` "ForDuration"))
        (if _returnvalue_2
          (for _array_element _outhits
            (bind _asbp_enemy (cast `/Game/HumanDenfense/BluePrint/Enemy/BP_Enemy` (`.HitActor` (`GameplayStatics.BreakHitResult` _array_element))))
            (`/Game/HumanDenfense/BluePrint/Enemy/BP_Enemy.Chaofeng` _asbp_enemy self (`self.Skill02Time`)))
          (set `self.Skill02Ready` false))
        (else
          (goto _label))))
    (:`3`
      (if (`self.Skill03Ready`)
        (`KismetSystemLibrary.K2_ClearAndInvalidateTimerHandle` (`self.Skill03Timer`))
        (bind _returnvalue_3 (`KismetSystemLibrary.K2_SetTimerDelegate` (delegate `Skill03Reset`) (`self.Skill03Delay`) true))
        (set `self.Skill03Timer` _returnvalue_3)
        (bind (_outhits_2 _returnvalue_4) (`KismetSystemLibrary.SphereTraceMultiForObjects` :`Start` _wordlocation_2 :`End` _wordlocation_2 :`Radius` (`self.Skill03Range`) :`ObjectTypes` (`|MakeArray` "ObjectTypeQuery8" :!type "EObjectTypeQuery Enum") :`DrawDebugType` "ForDuration"))
        (if _returnvalue_4
          (for _array_element_2 _outhits_2
            (bind _asbp_enemy_2 (cast `/Game/HumanDenfense/BluePrint/Enemy/BP_Enemy` (`.HitActor` (`GameplayStatics.BreakHitResult` _array_element_2))))
            (`/Game/HumanDenfense/BluePrint/Enemy/BP_Enemy.Jitui` _asbp_enemy_2 (* (`self.GetActorForwardVector` _asbp_enemy_2) (`self.Skill03Destance`)))
            (`GameplayStatics.ApplyDamage` _asbp_enemy_2 (`self.NomalDamage`) null self))
          (set `self.Skill03Ready` false)
          (`KismetSystemLibrary.PrintString` "Skill03"))
        (elif (`self.Skill02Ready`)
          (goto _label_2)
          (else
            (goto _label)))))))

(event `self.Skill02`
  (`/Engine/EditorBlueprintResources/StandardMacros.DoOnce` false
    (:`Completed`
      (set `self.SkillLevel` 2)
      (bind _returnvalue (`KismetSystemLibrary.K2_SetTimerDelegate` (delegate `Skill02Reset`) (`self.Skill02Delay`) true))
      (set `self.Skill02Timer` _returnvalue)
      (`KismetSystemLibrary.PrintString` "Skill02"))))

(event `Skill02Reset`
  (set `self.Skill02Ready` true))

(event `self.Skill03`
  (`/Engine/EditorBlueprintResources/StandardMacros.DoOnce` false
    (:`Completed`
      (set `self.SkillLevel` 3)
      (bind _returnvalue (`KismetSystemLibrary.K2_SetTimerDelegate` (delegate `Skill03Reset`) (`self.Skill03Delay`) true))
      (set `self.Skill03Timer` _returnvalue))))

(event `Skill03Reset`
  (set `self.Skill03Ready` true))

(fn `UserConstructionScript`
  (`parent.UserConstructionScript`))