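; Melee (JinZhan) attacker Blueprint in HumanDenfense that hits its first enemy with montage-timed normal attacks or a timer-recharged Skill01.
; Skill01 deals double radial damage around that enemy, with an IsTwice toggle driving a delayed repeat; hits feed CaculateHP through the HPjiqu factor.
; Skill02 raises damage, also setting HPjiqu at level 30, while Skill03 halves attack and skill delays.
; An older box-trace version of Skill01 remains unconnected.
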(event `self.Skill02`
  (if (== (`self.Level`) 30)
    (set `self.NomalDamage` (* (`self.NomalDamage`) 1.3))
    (set `self.HPjiqu` -0.3)
    (else
      (set `self.NomalDamage` (+ (* (`self.DamageUP`) 0.3) (`self.NomalDamage`)))
      (set `self.DamageUP` (* (`self.DamageUP`) 1.3)))))

(event `self.Skill03`
  (set `self.AttackDelay` (* (`self.AttackDelay`) 0.5))
  (set `self.Skill01Delay` (* (`self.Skill01Delay`) 0.5)))

(event `self.Skill01`
  ;[1 1 1] NormalAttackAndSkill01
  (bind _returnvalue (`KismetSystemLibrary.K2_SetTimerDelegate` (delegate `SkillReset`) (`self.Skill01Delay`) true))
  (set `self.Skill01Timer` _returnvalue))

(event `SkillReset`
  ;[1 1 1] NormalAttackAndSkill01
  (set `self.Skill01Ready?` true))

(event `self.AttackTo`
  (bind _ref_firstenemy (`self.Ref_FirstEnemy`))
  (bind _returnvalue (* (`self.NomalDamage`) 2.0))
  ;[1 1 1] NormalAttackAndSkill01
  (if (`self.Skill01Ready?`)
    (`KismetSystemLibrary.K2_ClearAndInvalidateTimerHandle` (`self.Skill01Timer`))
    (bind _returnvalue_2 (`KismetSystemLibrary.K2_SetTimerDelegate` (delegate `SkillReset`) (`self.Skill01Delay`) true))
    (set `self.Skill01Timer` _returnvalue_2)
    (`|PlayMontage` (`self.Mesh`) (`self.Ref_Montage`) 1.0 0.0 (`self.StartSection`)
      (:`then`
        (set `self.isAttacking` true))
      (:`OnCompleted`
        (set `self.isAttacking` false))
      (:`OnNotifyBegin`
        (`/Engine/EditorBlueprintResources/StandardMacros.IsValid` _ref_firstenemy :!label _label
          (:`Is Valid`
            (bind _returnvalue_3 (`GameplayStatics.ApplyRadialDamage` :`BaseDamage` _returnvalue :`Origin` (`self.K2_GetActorLocation` _ref_firstenemy) :`DamageRadius` (`self.SkillRadius`) :`DamageCauser` self :`InstigatedByController` null :`bDoFullDamage` true :`DamagePreventionChannel` "ECC_GameTraceChannel2"))
            (if _returnvalue_3
              (`KismetSystemLibrary.PrintString` (`KismetStringLibrary.Conv_DoubleToString` _returnvalue))
              (`self.CaculateHP` (* _returnvalue (`self.HPjiqu`)))
              (set `self.IsTwice` (not (`self.IsTwice`)))
              (if (`self.IsTwice`)
                (set `self.Skill01Ready?` false)
                (else
                  (`KismetSystemLibrary.Delay` 0.3)
                  (goto _label))))))))
    (else
      (`|PlayMontage` (`self.Mesh`) (`self.Ref_Montage`) 1.0 0.0 (`self.StartSection`)
        (:`then`
          (set `self.isAttacking` true))
        (:`OnCompleted`
          (set `self.isAttacking` false))
        (:`OnNotifyBegin`
          (`GameplayStatics.ApplyDamage` (`self.Ref_FirstEnemy`) (`self.NomalDamage`) null self)
          (`self.CaculateHP` (* (`self.NomalDamage`) (`self.HPjiqu`))))))))

(fn `UserConstructionScript`
  (`parent.UserConstructionScript`))