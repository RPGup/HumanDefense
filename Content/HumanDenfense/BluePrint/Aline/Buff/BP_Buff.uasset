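; BP_Buff is a support unit that heals and strengthens nearby allies and takes damage from enemies until destroyed.
; A sphere trace at BeginPlay caches allies in range (humans, gold makers, EXP uppers, other buffs).
; Experience raises stats up to a star-based level cap, unlocking a looping heal via negative CaculateHP, then a one-time HP multiplier on cached allies.
; A UI_Health widget shows health, experience, level and stars.
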(event `self.ReceiveBeginPlay`
  (bind _outactors (`GameplayStatics.GetAllActorsOfClass` "/Game/HumanDenfense/BluePrint/Aline/Base/BP_Base.BP_Base_C"))
  (set `self.Ref_Base` (`|GetArrayItem` _outactors))
  (set `self.wordlocation` (`self.K2_GetActorLocation`))
  (`self.SearchFriend`))

(event `SearchFriend`
  (bind _ref_alinesearched (`self.Ref_AlineSearched`))
  (bind _wordlocation (`self.wordlocation`))
  (bind (_outhits _returnvalue) (`KismetSystemLibrary.SphereTraceMultiForObjects` :`Start` _wordlocation :`End` _wordlocation :`Radius` (`self.BuffRange`) :`ObjectTypes` (`|MakeArray` "ObjectTypeQuery7" :!type "EObjectTypeQuery Enum") :`DrawDebugType` "ForDuration"))
  (if _returnvalue
    (`KismetArrayLibrary.Array_Clear` _ref_alinesearched)
    (for _array_element _outhits
      (`KismetArrayLibrary.Array_Add` _ref_alinesearched (`.HitActor` (`GameplayStatics.BreakHitResult` _array_element))))))

(event `LevelUp`
  (bind _asui_health (cast `/Game/HumanDenfense/UI/aLINE/UI_Health` (`WidgetComponent.GetUserWidgetObject` (`self.Widget`))))
  (set `/Game/HumanDenfense/UI/aLINE/UI_Health.Level` (`self.Level`) _asui_health)
  (set `self.HP` (+ (`self.HP`) (`self.HPUP`)))
  (set `self.MaxHp` (+ (`self.HPUP`) (`self.MaxHp`)))
  (set `self.AttackDamage` (+ (`self.DamageUp`) (`self.AttackDamage`)))
  (if (== (`self.Level`) 10)
    (bind _returnvalue (`KismetSystemLibrary.K2_SetTimerDelegate` (delegate `Skill01`) (`self.Skill01JianGe`) true))
    (set `self.Skill01Timer` _returnvalue)
    (elif (== (`self.Level`) 30)
      (`self.Skill02`)
      (elif (== (`self.Level`) 50)
        _))))

(event `Skill01`
  (bind _returnvalue (* (`self.AttackDamage`) -1.0))
  (for _array_element (`self.Ref_AlineSearched`)
    (bind _asbp_human (cast `/Game/HumanDenfense/BluePrint/Aline/Attack/BP_Human` _array_element)
      (:`then`
        (`/Game/HumanDenfense/BluePrint/Aline/Attack/BP_Human.CaculateHP` _asbp_human _returnvalue))
      (:`CastFailed`
        (bind _asbp_gold_maker_base (cast `/Game/HumanDenfense/BluePrint/Aline/GoldMaker/BP_GoldMakerBase` _array_element)
          (:`then`
            (`/Game/HumanDenfense/BluePrint/Aline/GoldMaker/BP_GoldMakerBase.CaculateHP` _asbp_gold_maker_base _returnvalue))
          (:`CastFailed`
            (bind _asbp_exp_uper_base (cast `/Game/HumanDenfense/BluePrint/Aline/ExpUper/BP_ExpUperBase` _array_element)
              (:`then`
                (`/Game/HumanDenfense/BluePrint/Aline/ExpUper/BP_ExpUperBase.CaculateHP` _asbp_exp_uper_base _returnvalue))
              (:`CastFailed`
                (bind _asbp_buff (cast `/Game/HumanDenfense/BluePrint/Aline/Buff/BP_Buff` _array_element))
                (`self.CaculateHP` _asbp_buff _returnvalue))))))))
  (`KismetSystemLibrary.PrintString` "huixueBUFF"))

(event `Skill02`
  (bind _skill02hpuptimes (`self.Skill02HPupTimes`))
  (bind _skill02hpuptimes_2 (`self.Skill02HPupTimes`))
  (bind _skill02hpuptimes_3 (`self.Skill02HPupTimes`))
  (bind _skill02hpuptimes_4 (`self.Skill02HPupTimes`))
  ;[1 1 1] 技能2
  (for _array_element (`self.Ref_AlineSearched`)
    (bind _asbp_human (cast `/Game/HumanDenfense/BluePrint/Aline/Attack/BP_Human` _array_element)
      (:`then`
        (set `/Game/HumanDenfense/BluePrint/Aline/Attack/BP_Human.HP` (* _skill02hpuptimes_2 (`/Game/HumanDenfense/BluePrint/Aline/Attack/BP_Human.HP` _asbp_human)) _asbp_human)
        (set `/Game/HumanDenfense/BluePrint/Aline/Attack/BP_Human.HPUP` (* (`/Game/HumanDenfense/BluePrint/Aline/Attack/BP_Human.HPUP` _asbp_human) _skill02hpuptimes_2) _asbp_human)
        (set `/Game/HumanDenfense/BluePrint/Aline/Attack/BP_Human.MaxHp` (* _skill02hpuptimes_2 (`/Game/HumanDenfense/BluePrint/Aline/Attack/BP_Human.MaxHp` _asbp_human)) _asbp_human))
      (:`CastFailed`
        (bind _asbp_gold_maker_base (cast `/Game/HumanDenfense/BluePrint/Aline/GoldMaker/BP_GoldMakerBase` _array_element)
          (:`then`
            (set `/Game/HumanDenfense/BluePrint/Aline/GoldMaker/BP_GoldMakerBase.HP` (* _skill02hpuptimes_3 (`/Game/HumanDenfense/BluePrint/Aline/GoldMaker/BP_GoldMakerBase.HP` _asbp_gold_maker_base)) _asbp_gold_maker_base)
            (set `/Game/HumanDenfense/BluePrint/Aline/GoldMaker/BP_GoldMakerBase.HPUP` (* _skill02hpuptimes_3 (`/Game/HumanDenfense/BluePrint/Aline/GoldMaker/BP_GoldMakerBase.HPUP` _asbp_gold_maker_base)) _asbp_gold_maker_base)
            (set `/Game/HumanDenfense/BluePrint/Aline/GoldMaker/BP_GoldMakerBase.MaxHp` (* _skill02hpuptimes_3 (`/Game/HumanDenfense/BluePrint/Aline/GoldMaker/BP_GoldMakerBase.MaxHp` _asbp_gold_maker_base)) _asbp_gold_maker_base))
          (:`CastFailed`
            (bind _asbp_exp_uper_base (cast `/Game/HumanDenfense/BluePrint/Aline/ExpUper/BP_ExpUperBase` _array_element)
              (:`then`
                (set `/Game/HumanDenfense/BluePrint/Aline/ExpUper/BP_ExpUperBase.HP` (* _skill02hpuptimes_4 (`/Game/HumanDenfense/BluePrint/Aline/ExpUper/BP_ExpUperBase.HP` _asbp_exp_uper_base)) _asbp_exp_uper_base)
                (set `/Game/HumanDenfense/BluePrint/Aline/ExpUper/BP_ExpUperBase.HPUP` (* (`/Game/HumanDenfense/BluePrint/Aline/ExpUper/BP_ExpUperBase.HPUP` _asbp_exp_uper_base) _skill02hpuptimes_4) _asbp_exp_uper_base)
                (set `/Game/HumanDenfense/BluePrint/Aline/ExpUper/BP_ExpUperBase.MaxHp` (* _skill02hpuptimes_4 (`/Game/HumanDenfense/BluePrint/Aline/ExpUper/BP_ExpUperBase.MaxHp` _asbp_exp_uper_base)) _asbp_exp_uper_base))
              (:`CastFailed`
                (bind _asbp_buff (cast `/Game/HumanDenfense/BluePrint/Aline/Buff/BP_Buff` _array_element))
                (set `/Game/HumanDenfense/BluePrint/Aline/Buff/BP_Buff.HP` (* _skill02hpuptimes (`/Game/HumanDenfense/BluePrint/Aline/Buff/BP_Buff.HP` _asbp_buff)) _asbp_buff)
                (set `/Game/HumanDenfense/BluePrint/Aline/Buff/BP_Buff.HPUP` (* _skill02hpuptimes (`/Game/HumanDenfense/BluePrint/Aline/Buff/BP_Buff.HPUP` _asbp_buff)) _asbp_buff)
                (set `/Game/HumanDenfense/BluePrint/Aline/Buff/BP_Buff.MaxHp` (* (`/Game/HumanDenfense/BluePrint/Aline/Buff/BP_Buff.MaxHp` _asbp_buff) _skill02hpuptimes) _asbp_buff)))))))))

(event `Star+`
  (if (not (== (`self.StarLevel`) 5))
    (bind _asui_health (cast `/Game/HumanDenfense/UI/aLINE/UI_Health` (`WidgetComponent.GetUserWidgetObject` (`self.Widget`))))
    (set `self.StarLevel` (+ (`self.StarLevel`) 1))
    (set `/Game/HumanDenfense/UI/aLINE/UI_Health.Star` (`self.StarLevel`) _asui_health)))

(event `self.ReceiveAnyDamage`
  (params (Damage :type "Float (single-precision)") (DamageType :type "DamageType Object Reference") (InstigatedBy :type "Controller Object Reference") (DamageCauser :type "Actor Object Reference"))
  (cast `/Game/HumanDenfense/BluePrint/Enemy/BP_Enemy` DamageCauser)
  (`self.CaculateHP` Damage))

(fn `CaculateExp`
  (params (exp :type Integer))
  (bind _exp (`self.Exp`))
  (if (== (* (`self.StarLevel`) 10) (`self.Level`))
    (`KismetSystemLibrary.PrintString` "CanNotGetExp")
    (else
      (set `self.Exp` (+ exp (`self.Exp`)))
      (if (>= _exp (`self.LevelExp`)) :!label _label
        (set `self.Exp` (- _exp (`self.LevelExp`)))
        (set `self.Level` (+ (`self.Level`) 1))
        (`self.LevelUP`)
        (if (== (* (`self.StarLevel`) 10) (`self.Level`))
          (set `self.Exp` 0)
          (else
            (goto _label))))
      (bind _asui_health (cast `/Game/HumanDenfense/UI/aLINE/UI_Health` (`WidgetComponent.GetUserWidgetObject` (`self.Widget`))))
      (`ProgressBar.SetPercent` (`/Game/HumanDenfense/UI/aLINE/UI_Health.ExpBar` _asui_health) (/ (`KismetMathLibrary.Conv_IntToDouble` (`self.Exp`)) (`KismetMathLibrary.Conv_IntToDouble` (`self.LevelExp`))))
      (return))))

(fn `CaculateHP`
  (params (NewParam :type "Float (double-precision)"))
  (bind _maxhp (`self.MaxHp`))
  (bind _output_get (set `self.HP` (- (`self.HP`) NewParam)))
  (bind _asui_health (cast `/Game/HumanDenfense/UI/aLINE/UI_Health` (`WidgetComponent.GetUserWidgetObject` (`self.Widget`))))
  (`ProgressBar.SetPercent` (`/Game/HumanDenfense/UI/aLINE/UI_Health.HealthBar` _asui_health) (/ _output_get (`self.MaxHp`)))
  (if (<= _output_get 0.0)
    (`self.K2_DestroyActor`)
    (`KismetSystemLibrary.PrintString` "death")
    (elif (>= (`self.HP`) _maxhp)
      (set `self.HP` _maxhp)))
  (return))

(fn `UserConstructionScript`)